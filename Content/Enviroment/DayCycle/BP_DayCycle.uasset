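; Day/night cycle actor that rotates the sky over a configurable day length in minutes.
; The SunCycle timeline, rate-scaled to that length, lerps Root through a full tilted pitch rotation and calls an empty StartDay event on each New Day.
; Optional flags randomise the starting pitch and start the cycle at BeginPlay.
; Construction copies post-process settings, and an AstroEvent macro provides a guarded counter decrement.
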(event `self.ReceiveBeginPlay`
  (if (`self.Random Start`)
    (`SceneComponent.K2_SetWorldRotation` (`self.Day and Night Cycle`) (`KismetMathLibrary.MakeRotator` 0.0 (`KismetMathLibrary.RandomFloatInRange` 0.0 360.0)) false false))
  (if (`self.StartCycle?`)
    (`TimelineComponent.SetPlayRate` (`self.Sun Cycle`) (/ 1.0 (* (`self.Day Length (Minutes)`) 60.0)))
    (bind (_direction _day) (`Timeline|Sun Cycle` :!via `PlayFromStart`)
      (:`Update`
        (`SceneComponent.K2_SetRelativeRotation` (`self.Root`) (`KismetMathLibrary.RLerp` (struct :`Yaw` 45.0) (struct :`Pitch` 360.0 :`Yaw` 45.0) _day) false false))
      (:`New Day`
        (`self.Start Day`)))))

(event `Start Day`)

(fn `UserConstructionScript`
  (set `PostProcessComponent.Settings` (`self.Settings`) (`self.PostProcess`)))