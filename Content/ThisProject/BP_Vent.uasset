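; BP_Vent is a vent actor whose static mesh can be knocked loose.
; Its Trigger event enables physics simulation on the mesh and applies a velocity-change impulse along the mesh's right vector with an upward lift, popping it off.
; The construction script sets the mesh's visibility from a Visible variable, and BeginPlay, overlap and Tick are unused.
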(event `self.Trigger`
  (params (Damage :type "/Game/ThisProject/Struct_DamageHitResult Structure"))
  (bind _staticmesh (`self.StaticMesh`))
  (`PrimitiveComponent.SetSimulatePhysics` _staticmesh true)
  (`PrimitiveComponent.AddImpulse` _staticmesh (+ (* (`SceneComponent.GetRightVector` _staticmesh) 400.0) (0.0 0.0 200.0)) "None" true))

(fn `UserConstructionScript`
  (`parent.UserConstructionScript`)
  (`SceneComponent.SetVisibility` (`self.StaticMesh`) (`self.Visible`) false))