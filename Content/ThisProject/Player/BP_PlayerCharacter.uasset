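; First-person player character that hubs components for weapons, powers, sanity/health, extra lives, inventory, vouchers and physics interaction.
; Input and gameplay events route to those components, with item tags selecting effects and stat upgrades adjusting component values.
; Sphere traces notify nearby AI and add insanity when looking at flagged surfaces.
; It also handles fall damage, a Wind-power air jump, hit feedback, and moving the camera onto a death actor.
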(event `self.ReceiveBeginPlay`
  (`parent.ReceiveBeginPlay`)
  (`self.Initialize Components`)
  (`KismetSystemLibrary.K2_SetTimerDelegate` (`|CreateDelegate` :!event `Check Proximity`) 1.0 true)
  (`KismetSystemLibrary.K2_SetTimerDelegate` (`|CreateDelegate` :!event `CheckSight`) 0.5 true))

(event `Check Proximity`
  (bind _returnvalue (`SceneComponent.K2_GetComponentLocation` (`self.FirstPersonCamera`)))
  (bind _outhit (`KismetSystemLibrary.SphereTraceSingle` _returnvalue (- _returnvalue (0.0 0.0 1.0)) 1250.0 "TraceTypeQuery4"))
  (message `/Game/Base/BPI_AI.AI Proximity` (`.HitActor` (`GameplayStatics.BreakHitResult` _outhit))))

(event `EnhancedInput|/Game/BaseCharacter/Input/Actions/IA_Attack`
  (params (ActionValue :type Boolean) (ElapsedSeconds :type "Float (double-precision)") (TriggeredSeconds :type "Float (double-precision)") (InputAction :type "InputAction Object Reference" :default "/Game/BaseCharacter/Input/Actions/IA_Attack.IA_Attack"))
  (:`Started`
    (`/Game/ThisProject/Player/Comp_Weapon.Use Weapon` (`self.Comp_Weapon`))))

(event `EnhancedInput|/Game/BaseCharacter/Input/Actions/IA_Crouch`
  (params (ActionValue :type Boolean) (ElapsedSeconds :type "Float (double-precision)") (TriggeredSeconds :type "Float (double-precision)") (InputAction :type "InputAction Object Reference" :default "/Game/BaseCharacter/Input/Actions/IA_Crouch.IA_Crouch"))
  (:`Started`
    (`self.Event Crouch`))
  (:`Completed`
    (`self.Event Uncrouch`)))

(event `EnhancedInput|/Game/BaseCharacter/Input/Actions/IA_Interact`
  (params (ActionValue :type Boolean) (ElapsedSeconds :type "Float (double-precision)") (TriggeredSeconds :type "Float (double-precision)") (InputAction :type "InputAction Object Reference" :default "/Game/BaseCharacter/Input/Actions/IA_Interact.IA_Interact"))
  (:`Started`
    (bind _cable (`self.Cable`)
      (:`then`
        (message `/Game/ThisProject/Interactables/BPI_Interact.Interact` _cable self (`self.Interacting Component`))
        (set `self.Cable` null))
      (:`else`
        (`/Game/ThisProject/Comp_PhysicsInteractor.Interact` (`self.Comp_PhysicsInteractor`))))))

(event `EnhancedInput|/Game/BaseCharacter/Input/Actions/IA_Power`
  (params (ActionValue :type Boolean) (ElapsedSeconds :type "Float (double-precision)") (TriggeredSeconds :type "Float (double-precision)") (InputAction :type "InputAction Object Reference" :default "/Game/BaseCharacter/Input/Actions/IA_Power.IA_Power"))
  (:`Started`
    (`/Game/ThisProject/Player/Comp_Power.Use Power` (`self.Comp_Power`))))

(event `/Game/ThisProject/Player/BPI_Interactor.Player Cable`
  (params (Cable :type "/Game/ThisProject/Interactables/Power/BP_PlayerCable Object Reference"))
  (set `self.Cable` Cable))

(event `self.Comp_ExtraLife.On All Lives Lost`
  (bind _returnvalue (`|CreateWidget` "/Game/ThisProject/Player/DeathScreen/WB_DeathScreen.WB_DeathScreen_C"))
  (`UserWidget.AddToViewport` _returnvalue 0)
  (`SceneComponent.K2_DetachFromComponent` (`self.FirstPersonCamera`) "KeepWorld" "KeepWorld" "KeepWorld" true)
  (`SceneComponent.SetVisibility` (`self.FirstPersonMesh`) false true)
  (bind _returnvalue_2 (`|SpawnActorFromClass` "/Game/ThisProject/Player/DeathScreen/BP_DeathActor.BP_DeathActor_C" (`SceneComponent.K2_GetComponentToWorld` (`self.FirstPersonCamera`)) "Undefined" "MultiplyWithRoot" null null))
  (`SceneComponent.K2_AttachToComponent` (`self.FirstPersonCamera`) (`/Game/ThisProject/Player/DeathScreen/BP_DeathActor.Sphere` _returnvalue_2) "None" "SnapToTarget" "SnapToTarget" "SnapToTarget" true))

(event `self.Comp_SanityHealth.On Death`
  (bind _comp_sanityhealth (`self.Comp_SanityHealth`))
  (bind _comp_extralife (`self.Comp_ExtraLife`))
  (`/Game/ThisProject/Player/Comp_ExtraLife.Life Lost` _comp_extralife)
  (if (!= (`/Game/ThisProject/Player/Comp_ExtraLife.ExtraLives` _comp_extralife) 0)
    (`/Game/ThisProject/Player/Comp_PlayerHealth.Insanity Lost` _comp_sanityhealth (`/Game/ThisProject/Player/Comp_PlayerHealth.Current Insanity` _comp_sanityhealth))
    (`/Game/ThisProject/Player/Comp_PlayerHealth.Damage Lost` _comp_sanityhealth (`/Game/ThisProject/Player/Comp_PlayerHealth.Current Damage` _comp_sanityhealth))))

(event `/Game/ThisProject/Player/BPI_Interactor.Loot Vouchers`
  (params (Amount :type Integer))
  (`/Game/ThisProject/Player/Comp_VoucherPouch.Add Voucher` (`self.Comp_VoucherPouch`) Amount))

(event `self.OnLanded`
  (params (Hit :type "HitResult Structure (by ref)"))
  (bind _returnvalue (- (`KismetMathLibrary.Abs` (.z (`MovementComponent.Velocity` (`self.CharacterMovement`)))) (`CharacterMovementComponent.JumpZVelocity` (`self.CharacterMovement`)) 1000.0))
  (`parent.OnLanded` Hit)
  (set `/Game/ThisProject/Player/Comp_Power.Wind Jump Available?` true (`self.Comp_Power`))
  (if (> _returnvalue 0.0)
    (`self.Apply Damage` (make `/Game/ThisProject/Struct_DamageHitResult` (/ _returnvalue 100.0) (struct :`Time` 1.0 :`Location` (0.0 0.0 0.0) :`ImpactPoint` (0.0 0.0 0.0) :`Normal` (0.0 0.0 0.0) :`ImpactNormal` (0.0 0.0 0.0) :`TraceStart` (0.0 0.0 0.0) :`TraceEnd` (0.0 0.0 0.0) :`MyItem` -1 :`HitObjectHandle` (struct)) (struct :`GameplayTags` (struct :`(TagName` "DamageSource.Environment")))))
    (`/Engine/EditorBlueprintResources/StandardMacros.DoOnce` false
      (:`Completed`
        (message `/Game/ThisProject/Player/BPI_GameInstance.Play Doug Line` (`GameplayStatics.GetGameInstance`) "/Game/ThisProject/Assets_Imports/Doug/Voicelines/Doug_FallingDamage.Doug_FallingDamage")))))

(event `CheckSight`
  (bind _firstpersoncamera (`self.FirstPersonCamera`))
  (bind _returnvalue (`SceneComponent.K2_GetComponentLocation` _firstpersoncamera))
  (bind (_outhit _returnvalue_2) (`KismetSystemLibrary.SphereTraceSingle` _returnvalue (+ (* (`SceneComponent.GetForwardVector` _firstpersoncamera) 2500.0) _returnvalue) 25.0 "TraceTypeQuery1"))
  (if _returnvalue_2
    (if (`|EnumEquality` (`PhysicalMaterial.SurfaceType` (`.PhysMat` (`GameplayStatics.BreakHitResult` _outhit))) "SurfaceType1")
      (`/Game/ThisProject/Player/Comp_PlayerHealth.Insanity Gained` (`self.Comp_SanityHealth`) 0.1))))

(event `/Game/ThisProject/Player/BPI_Interactor.Upgrade Stat`
  (params (Stat :type "/Game/ThisProject/Player/Upgrades/Enum_PlayerStat Enum" :default "NewEnumerator5"))
  (bind _stats (`self.Stats`))
  (bind _comp_sanityhealth (`self.Comp_SanityHealth`))
  (bind _comp_weapon (`self.Comp_Weapon`))
  (bind _charactermovement (`self.CharacterMovement`))
  (`BlueprintMapLibrary.Map_Add` _stats Stat (+ (`BlueprintMapLibrary.Map_Find` _stats Stat) 1))
  (switch `/Game/ThisProject/Player/Upgrades/Enum_PlayerStat` Stat
    (:`NewEnumerator0`
      (set `/Game/ThisProject/Player/Comp_PlayerHealth.Max Health` (+ (`/Game/ThisProject/Player/Comp_PlayerHealth.Max Health` _comp_sanityhealth) 1.0) _comp_sanityhealth)
      (`/Game/ThisProject/Player/Comp_PlayerHealth.Health Gained` _comp_sanityhealth 1.0))
    (:`NewEnumerator1`
      (set `/Game/ThisProject/Player/Comp_Weapon.Damage Bonus` (+ (`/Game/ThisProject/Player/Comp_Weapon.Damage Bonus` _comp_weapon) 1.0) _comp_weapon))
    (:`NewEnumerator2`
      (set `/Game/ThisProject/Player/Comp_Weapon.Attack Speed` (+ (`/Game/ThisProject/Player/Comp_Weapon.Attack Speed` _comp_weapon) 0.1) _comp_weapon))
    (:`NewEnumerator4`
      (set `CharacterMovementComponent.MaxWalkSpeed` (+ (`CharacterMovementComponent.MaxWalkSpeed` _charactermovement) 100.0) _charactermovement))))

(event `self.Comp_Power1.On Animation Ended`
  (set `self.IsBusy` false :!label _label))

(event `self.Comp_Cig.On Animation Ended`
  (goto _label))

(event `self.Comp_Power.On Animation Ended`
  (goto _label))

(fn `Apply Damage`
  (params (`Damage Info` :type "/Game/ThisProject/Struct_DamageHitResult Structure"))
  (returns (Success :type Boolean))
  (bind (_damage _hitresult) (break `/Game/ThisProject/Struct_DamageHitResult` `Damage Info`))
  (bind (_bblockinghit _binitialoverlap _time _distance _location _impactpoint _normal _impactnormal) (`GameplayStatics.BreakHitResult` _hitresult))
  (message `/Game/ThisProject/Player/BPI_GameInstance.Save Hi-Score Damage Taken` (`GameplayStatics.GetGameInstance`) _damage)
  (`/Game/ThisProject/Player/Comp_PlayerHealth.Damage Gained` (`self.Comp_SanityHealth`) _damage)
  (`PlayerCameraManager.StartCameraShake` :`self` (`GameplayStatics.GetPlayerCameraManager` 0) :`ShakeClass` "/Game/ThisProject/Player/LCS_Impact.LCS_Impact_C" :`Scale` 2.0)
  (`GameplayStatics.PlaySoundAtLocation` "/Game/ThisProject/Materials/PhysicalMats/MSS_Impact_Body.MSS_Impact_Body" (`self.K2_GetActorLocation`) (struct) 1.0 1.0 0.0 null null null null)
  (`NiagaraFunctionLibrary.SpawnSystemAtLocation` "/Game/ThisProject/Materials/PhysicalMats/NS_Impact_Body.NS_Impact_Body" _impactpoint (`KismetMathLibrary.Conv_VectorToRotator` _impactnormal))
  (bind _returnvalue (`|CreateWidget` "/Game/ThisProject/Player/WB_Hit.WB_Hit_C"))
  (`UserWidget.AddToViewport` _returnvalue 0)
  (return false))

(fn `CanJumpInternal`
  (returns (ReturnValue :type Boolean))
  (bind _comp_power (`self.Comp_Power`))
  (if (`NavMovementComponent.IsFalling` (`self.CharacterMovement`))
    (bind _power (`/Game/ThisProject/Player/Comp_Power.Power` _comp_power)
      (:`then`
        (if (and (== (`/Game/ThisProject/Player/DA_PowerData.Tag` _power) (struct :`TagName` "Powers.Wind")) (`/Game/ThisProject/Player/Comp_Power.Wind Jump Available?` _comp_power))
          (`/Game/ThisProject/Player/Comp_Power.Wind Jump` (`self.Comp_Power`))
          (return false)
          (else
            _)))
      (:`else`
        _))
    (return false)
    (else
      (bind _returnvalue (`parent.CanJumpInternal`))
      (return _returnvalue))))

(fn `Check and Pay Cost`
  (params (Cost :type Integer))
  (returns (Success :type Boolean))
  (bind _success (`/Game/ThisProject/Player/Comp_VoucherPouch.Use Voucher` (`self.Comp_VoucherPouch`) Cost))
  (if _success
    (return _success)
    (else
      (bind _returnvalue (`|CreateWidget` "/Game/ThisProject/Player/WB_Announcment.WB_Announcment_C" null "You Cannot Afford This!"))
      (`UserWidget.AddToViewport` _returnvalue 0)
      (return false))))

(fn `Debug_TestDamage`
  (params (Radius :type "Float (single-precision)" :default 15.0) (TraceChannel :type "ETraceTypeQuery Enum" :default "TraceTypeQuery1") (Damage :type "Float (double-precision)") (`Hit Tags` :type "GameplayTagContainer Structure"))
  (bind _firstpersoncamera (`self.FirstPersonCamera`))
  (bind _returnvalue (`SceneComponent.K2_GetComponentLocation` _firstpersoncamera))
  (bind (_outhit _returnvalue_2) (`KismetSystemLibrary.SphereTraceSingle` :`Start` _returnvalue :`End` (`/Game/Base/BFL_General.Convert Trace` _returnvalue (`SceneComponent.GetForwardVector` _firstpersoncamera) 10000.0) :`Radius` Radius :`TraceChannel` TraceChannel :`DrawDebugType` "ForDuration"))
  (`/Game/Base/BFL_General.Apply Impulse to Hit` _outhit (* Damage 100.0))
  (if _returnvalue_2
    (message `/Game/ThisProject/BPI_Health.Apply Damage` (`.HitActor` (`GameplayStatics.BreakHitResult` _outhit)) (make `/Game/ThisProject/Struct_DamageHitResult` Damage _outhit `Hit Tags`))))

(fn `Debug_TestInteract`
  (bind _outhit (`self.Debug_TestTrace` 15.0 "TraceTypeQuery1" 200.0))
  (message `/Game/ThisProject/Interactables/BPI_Interact.Interact` (`.HitActor` (`GameplayStatics.BreakHitResult` _outhit)) self (`self.Interacting Component`)))

(fn `Debug_TestTrace`
  (params (Radius :type "Float (single-precision)" :default 15.0) (TraceChannel :type "ETraceTypeQuery Enum" :default "TraceTypeQuery1") (Distance :type "Float (double-precision)" :default 300.0))
  (returns (OutHit :type "HitResult Structure"))
  (bind _firstpersoncamera (`self.FirstPersonCamera`))
  (bind _returnvalue (`SceneComponent.K2_GetComponentLocation` _firstpersoncamera))
  (bind _outhit (`KismetSystemLibrary.SphereTraceSingle` :`Start` _returnvalue :`End` (`/Game/Base/BFL_General.Convert Trace` _returnvalue (`SceneComponent.GetForwardVector` _firstpersoncamera) Distance) :`Radius` Radius :`TraceChannel` TraceChannel :`DrawDebugType` "ForDuration"))
  (return _outhit))

(fn `Get Stat`
  (params (Stat :type "/Game/ThisProject/Player/Upgrades/Enum_PlayerStat Enum" :default "NewEnumerator5"))
  (returns (Value :type Integer))
  (return (`BlueprintMapLibrary.Map_Find` (`self.Stats`) Stat)))

(fn `Initialize Components`
  (bind _comp_sanityhealth (`self.Comp_SanityHealth`))
  (bind _firstpersonmesh (`self.FirstPersonMesh`))
  (`/Game/ThisProject/Comp_PhysicsInteractor.Initialize Interactor` (`self.Comp_PhysicsInteractor`) (`self.Interacting Component`) (`self.FirstPersonMesh`))
  (`/Game/ThisProject/Player/Comp_Power.Initialize Power` (`self.Comp_Power`) (`self.FirstPersonMesh`) (`self.Comp_SanityHealth`) (`self.FirstPersonCamera`) (`self.Comp_PhysicsInteractor`) (`self.Comp_ExtraLife`))
  (`/Game/ThisProject/Player/Comp_Weapon.Initialize Weapon` (`self.Comp_Weapon`) (`self.FirstPersonMesh`) (`self.FirstPersonCamera`))
  (`/Game/ThisProject/Player/Comp_Power.Initialize Power` (`self.Comp_Power1`) _firstpersonmesh _comp_sanityhealth (`self.FirstPersonCamera`) (`self.Comp_PhysicsInteractor`) (`self.Comp_ExtraLife`))
  (`/Game/ThisProject/Player/Comp_Cig.Initialize Cigs` (`self.Comp_Cig`) _firstpersonmesh _comp_sanityhealth (`self.FirstPersonCamera`))
  (`SkinnedMeshComponent.HideBoneByName` (`self.FirstPersonMesh`) "f_index_01_L_001" "PBO_None"))

(fn `IsPlayerBusy?`
  (returns (`IsBusy?` :type Boolean))
  (return (`self.IsBusy`)))

(fn `Loot Weapon`
  (params (Weapon :type "/Game/ThisProject/Player/DA_Weapon Object Reference"))
  (returns (success :type Boolean))
  (`/Game/ThisProject/Player/Comp_Weapon.Trade Weapon` (`self.Comp_Weapon`) Weapon)
  (set `self.HasWeapon?` true)
  (return false))

(fn `Pick Up Item`
  (params (Object :type "Actor Object Reference") (Item :type "/Game/GridInventory/Data/ST_Item Structure"))
  (returns (Return :type Boolean))
  (bind _success (`/Game/GridInventory/Comp_Inventory.PickUpItem` (`self.Comp_Inventory`) Object Item))
  (return _success))

(fn `Use Item`
  (params (Item :type "/Game/GridInventory/Data/DA_Items Object Reference"))
  (returns (Success :type Boolean))
  (`|ExecutionSequence`
    (:`then_0`
      (`/Engine/EditorBlueprintResources/StandardMacros.IsValid` Item
        (:`Is Valid`
          (for _array_element (`BlueprintGameplayTagLibrary.BreakGameplayTagContainer` (`/Game/GridInventory/Data/DA_Items.Uses` Item))
            (`|SwitchGameplayTag` _array_element
              (:`ItemEffects.WindPower`
                (`/Game/ThisProject/Player/Comp_Power.Trade Power` (`self.Comp_Power`) "/Game/ThisProject/Player/DA_Svento.DA_Svento")
                (set `self.IsBusy` true))
              (:`ItemEffects.GainSanity`
                (`/Game/ThisProject/Player/Comp_Cig.Use Cig` (`self.Comp_Cig`))
                (set `self.IsBusy` true))
              (:`ItemEffects.GainHealth`
                (`/Game/ThisProject/Player/Comp_Cig.Use Medkit` (`self.Comp_Cig`))
                (set `self.IsBusy` true))
              (:`ItemEffects.GainExtraLife`
                (`/Game/ThisProject/Player/Comp_Power.Trade Power` (`self.Comp_Power1`) "/Game/ThisProject/Player/DA_SecondHeart.DA_SecondHeart")
                (set `self.IsBusy` true))
              (:`ItemEffects.GainVouchers`
                (`self.Loot Vouchers` (`KismetMathLibrary.RandomIntegerInRange` 5 15))))))))
    (:`then_1`
      (return (`self.IsBusy`)))))

(fn `UserConstructionScript`
  (`parent.UserConstructionScript`))