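; BP_DestructableWall is a wall that breaks apart when triggered by damage tagged as explosive.
; The first such hit removes its Box and Decal components and enables physics on the Geometry Collection.
; It then crumbles a fixed range of clusters and launches each along the Arrow's forward direction, using ConvertTrace with a random angle to vary the velocity.
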(event `self.Trigger`
  (params (Damage :type "/Game/ThisProject/Struct_DamageHitResult Structure"))
  (bind _geometrycollection (`self.GeometryCollection`))
  (if (`BlueprintGameplayTagLibrary.HasTag` (`.HitTags_27_D428CAB14F1B0F3F4E170AB43135486C` (break `/Game/ThisProject/Struct_DamageHitResult` Damage)) (struct :`TagName` "DamageTypes.Explosive") true)
    (`/Engine/EditorBlueprintResources/StandardMacros.DoOnce` false
      (:`Completed`
        (`ActorComponent.K2_DestroyComponent` (`self.Box`))
        (`ActorComponent.K2_DestroyComponent` (`self.Decal`))
        (`PrimitiveComponent.SetSimulatePhysics` (`self.GeometryCollection`) true)
        (for _index (range 1 21)
          (`GeometryCollectionComponent.CrumbleCluster` _geometrycollection _index)
          (`GeometryCollectionComponent.ApplyLinearVelocity` _geometrycollection _index (`/Game/Base/BFL_General.Convert Trace` (1.0 1.0 1.0) (`SceneComponent.GetForwardVector` (`self.Arrow`)) 500.0 (`KismetMathLibrary.RandomFloatInRange` 0.0 45.0))))))))

(fn `UserConstructionScript`)