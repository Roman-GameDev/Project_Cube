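; Cultist melee enemy Blueprint that extends its parent's damage handling and adds attack, stumble, death and voice line behavior.
; Attacks play a random montage whose notify fires a forward sphere trace from Sight to damage the hit actor.
; Taking damage triggers a hit-reaction stumble that halts movement.
; Death removes props, hides the head bone and spawns a head explosion, while Ramble randomly plays voice lines and BeginPlay starts a randomized looping timer.
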(event `self.ReceiveBeginPlay`
  (`parent.ReceiveBeginPlay`)
  (`KismetSystemLibrary.K2_SetTimerDelegate` (`|CreateDelegate` :!event `Ramble`) (`KismetMathLibrary.RandomFloatInRange` 10.0 20.0) true))

(event `self.Attack`
  (bind _sight (`self.Sight`))
  (bind _returnvalue (`SceneComponent.K2_GetComponentLocation` _sight))
  (`|PlayMontage` (`self.SkeletalMeshComponentBudgeted`) (`KismetArrayLibrary.Array_Random` (`self.Attacks`))
    (:`OnNotifyBegin`
      (bind (_outhit _returnvalue_2) (`KismetSystemLibrary.SphereTraceSingleForObjects` :`Start` _returnvalue :`End` (+ _returnvalue (* (`SceneComponent.GetForwardVector` _sight) 75.0)) :`Radius` 70.0 :`ObjectTypes` (`|MakeArray` "ObjectTypeQuery7" :!type "EObjectTypeQuery Enum") :`DrawDebugType` "ForDuration"))
      (if _returnvalue_2
        (message `/Game/ThisProject/BPI_Health.Apply Damage` (`.HitActor` (`GameplayStatics.BreakHitResult` _outhit)) (make `/Game/ThisProject/Struct_DamageHitResult` 1.25 _outhit (struct :`GameplayTags` (struct :`(TagName` "DamageSource.Enemy")))))))))

(event `self.Death`
  (bind _skeletalmeshcomponentbudgeted (`self.SkeletalMeshComponentBudgeted`))
  (`ActorComponent.K2_DestroyComponent` (`self.Cig`))
  (`ActorComponent.K2_DestroyComponent` (`self.Crowbar`))
  (`ActorComponent.K2_DestroyComponent` (`self.Niagara`))
  (`SkinnedMeshComponent.HideBoneByName` _skeletalmeshcomponentbudgeted "head" "PBO_None")
  (`NiagaraFunctionLibrary.SpawnSystemAtLocation` "/Game/ThisProject/Assets_Imports/Character/Enemy/NS_HeadExplosion.NS_HeadExplosion" (`SceneComponent.GetSocketLocation` _skeletalmeshcomponentbudgeted "head")))

(event `Ramble`
  (if (`KismetMathLibrary.RandomBool`)
    (`self.Play Voiceline` (`KismetArrayLibrary.Array_Random` (`self.Rambles`)))))

(event `Stumble`
  (`|PlayMontage` (`self.SkeletalMeshComponentBudgeted`) "/Game/ThisProject/Enemy/RetargettedAnimations/AS_Cultist_HitReaction_Montage.AS_Cultist_HitReaction_Montage"
    (:`then`
      (`MovementComponent.StopMovementImmediately` (`self.CharacterMovement`)))))

(fn `Apply Damage`
  (params (`Damage Info` :type "/Game/ThisProject/Struct_DamageHitResult Structure"))
  (returns (Success :type Boolean))
  (bind _success (`parent.Apply Damage` `Damage Info`))
  (`self.Stumble`)
  (return _success))

(fn `UserConstructionScript`
  (`parent.UserConstructionScript`))