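; BP_Cultist_First is a cultist enemy variant, apparently the first one encountered, that layers a delayed start and a post-kill voice line onto its parent class.
; BeginPlay sets a short timer to an Init event, which only then calls the parent BeginPlay, postponing inherited setup.
; Death passes through a DoOnce, sends the Doug_PostEnemy line message to the game instance, then runs the parent death logic.
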(event `self.ReceiveBeginPlay`
  (`KismetSystemLibrary.K2_SetTimerDelegate` (delegate `Init`) 2.5))

(event `Init`
  (`parent.ReceiveBeginPlay`))

(event `self.Death`
  (`/Engine/EditorBlueprintResources/StandardMacros.DoOnce` false
    (:`Completed`
      (message `/Game/ThisProject/Player/BPI_GameInstance.Play Doug Line` (`GameplayStatics.GetGameInstance`) "/Game/ThisProject/Assets_Imports/Doug/Voicelines/Done/Doug_PostEnemy.Doug_PostEnemy")
      (`parent.Death`))))

(fn `UserConstructionScript`
  (`parent.UserConstructionScript`))