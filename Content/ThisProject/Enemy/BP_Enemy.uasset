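; BP_Enemy is an AI enemy that chases the player, takes damage through a health component and ragdolls when health empties.
; A proximity event starts a looping sight timer that tests tiered angle and distance thresholds, comparing both actors' forward vectors rather than direction to target.
; A passed check triggers AI movement toward the player, re-issued after each success or failure.
; Checking stops when the player is out of range.
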(event `self.ReceiveBeginPlay`
  (set `self.Target` (`GameplayStatics.GetPlayerCharacter` 0)))

(event `self.Comp_Health.On Resource Emptied`
  (`PrimitiveComponent.SetSimulatePhysics` (`self.SkeletalMeshComponentBudgeted`) true))

(event `/Game/Base/BPI_AI.AI Proximity`
  (`self.Start Checking Sight`))

(event `Start Checking Sight`
  (`KismetSystemLibrary.K2_SetTimerDelegate` (delegate `Check Sight`) 0.2 true)
  (goto _label :!via `Reset`))

(event `Check Sight`
  (if (or (`self.Sight Check` -0.7 2500.0) (`self.Sight Check` -0.5 1250.0) (`self.Sight Check` -0.05 400.0) (`self.Sight Check` 1.0 75.0))
    (`KismetSystemLibrary.K2_ClearTimer` null "Check Sight")
    (`/Engine/EditorBlueprintResources/StandardMacros.DoOnce` false :!label _label
      (:`Completed`
        (`self.Move Towards Target`)))
    (elif (not (< (`self.Get Distance to Target`) 2600.0))
      (`KismetSystemLibrary.K2_ClearTimer` null "Check Sight"))))

(event `Move Towards Target`
  (`|AIMoveTo` self (0.0 0.0 0.0) (`self.Target`) 200.0
    (:`OnSuccess`
      _)
    (:`OnFail`
      _))
  (`KismetSystemLibrary.K2_SetTimerDelegate` (delegate `Move Towards Target`) 1.0))

(fn `Apply Damage`
  (params (`Damage Info` :type "/Game/ThisProject/Struct_DamageHitResult Structure"))
  (returns (Success :type Boolean))
  (`/Game/ThisProject/Comp_Health.Apply Damage to Health` (`self.Comp_Health`) `Damage Info`)
  (return true))

(fn `Get Distance to Target`
  (returns (ReturnValue :type "Float (double-precision)"))
  (return (`KismetMathLibrary.Vector_Distance` (`self.K2_GetActorLocation` (`self.Target`)) (`self.K2_GetActorLocation`))))

(fn `Sight Check`
  (params (Angle :type "Float (double-precision)") (Distance :type "Float (double-precision)"))
  (returns (ReturnValue :type Boolean))
  (return (and (< (`KismetMathLibrary.Dot_VectorVector` (`self.GetActorForwardVector`) (`self.GetActorForwardVector` (`self.Target`))) Angle) (< (`self.Get Distance to Target`) Distance))))

(fn `UserConstructionScript`)