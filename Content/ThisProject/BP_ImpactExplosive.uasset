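; BP_ImpactExplosive is a damageable physics object that explodes on a hard impact once primed.
; ApplyDamage starts a short timer, and the Prime event sets the Damaged flag that enables the hit check.
; When a component hit passes the velocity threshold, it explodes once and destroys itself.
; The explosion spawns a Niagara effect, then uses a radial trace to send player-tagged damage and apply impulses.
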(event `self.StaticMesh.OnComponentHit`
  (params (HitComponent :type "PrimitiveComponent Object Reference") (OtherActor :type "Actor Object Reference") (OtherComp :type "PrimitiveComponent Object Reference") (NormalImpulse :type "Vector Structure") (Hit :type "HitResult Structure (by ref)"))
  (if (`self.Damaged`)
    (bind _returnvalue (`PrimitiveComponent.GetPhysicsLinearVelocity` (`self.StaticMesh`) "None"))
    (if (> (`KismetMathLibrary.FCeil` (/ (`KismetMathLibrary.VSize` _returnvalue) 10.0)) 20)
      (`/Engine/EditorBlueprintResources/StandardMacros.DoOnce` false
        (:`Completed`
          (`self.Explode`)
          (`self.K2_DestroyActor`))))))

(event `Prime`
  (set `self.Damaged` true))

(event `Explode`
  (`NiagaraFunctionLibrary.SpawnSystemAtLocation` "/Game/ThisProject/NS_Explosion.NS_Explosion" (`SceneComponent.K2_GetComponentLocation` (`self.StaticMesh`)))
  (bind _hits_result (`/Game/Base/BFL_General.Explosion Trace` (`SceneComponent.K2_GetComponentLocation` (`self.StaticMesh`)) 300.0 "TraceTypeQuery1" "None" (`|MakeArray` self :!type "Actor Object Reference")))
  (for _array_element _hits_result
    (message `/Game/ThisProject/BPI_Health.Apply Damage` (`.HitActor` (`GameplayStatics.BreakHitResult` _array_element)) (make `/Game/ThisProject/Struct_DamageHitResult` 10.0 _array_element (struct :`GameplayTags` (struct :`(TagName` "DamageSource.Player") :`(TagName` "DamageTypes.Explosive")))))
    (`/Game/Base/BFL_General.Apply Impulse to Hit` _array_element 1000.0)))

(fn `Apply Damage`
  (params (`Damage Info` :type "/Game/ThisProject/Struct_DamageHitResult Structure"))
  (returns (Success :type Boolean))
  (`parent.Apply Damage` `Damage Info`)
  (`KismetSystemLibrary.K2_SetTimerDelegate` (`|CreateDelegate` :!event `Prime`) 0.2)
  (return true))

(fn `UserConstructionScript`
  (`parent.UserConstructionScript`))