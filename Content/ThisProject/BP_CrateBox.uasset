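; BP_CrateBox is a loot crate that pops open once when its Trigger event fires, ignoring the damage value passed in.
; The lid starts simulating physics, is thrown off with linear and angular impulses, detaches and ignores a game trace channel.
; It then spawns a small random number of BP_Lootable_Item actors at ItemSpawn, each given random CrateItemPool data and an upward impulse.
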(event `self.Trigger`
  (params (Damage :type "/Game/ThisProject/Struct_DamageHitResult Structure"))
  (bind _lid (`self.Lid`))
  (`/Engine/EditorBlueprintResources/StandardMacros.DoOnce` false
    (:`Completed`
      (`PrimitiveComponent.SetSimulatePhysics` _lid true)
      (`PrimitiveComponent.AddImpulse` _lid (0.0 200.0 300.0) "None" true)
      (`PrimitiveComponent.AddAngularImpulseInDegrees` _lid (15.0 90.0 15.0) "None" true)
      (`SceneComponent.K2_DetachFromComponent` _lid "KeepWorld" "KeepWorld" "KeepWorld" true)
      (`PrimitiveComponent.SetCollisionResponseToChannel` (`self.Lid`) "ECC_GameTraceChannel3" "ECR_Ignore")
      (for _ (range 1 (+ (`KismetMathLibrary.RandomIntegerInRange` 1 3) 1))
        (bind _returnvalue (`|SpawnActorFromClass` "/Game/ThisProject/Interactables/BP_Lootable_Item.BP_Lootable_Item_C" (`SceneComponent.K2_GetComponentToWorld` (`self.ItemSpawn`)) "Undefined" "MultiplyWithRoot" null (struct) (`KismetArrayLibrary.Array_Random` (`self.Crate Item Pool`)) "/Engine/BasicShapes/Cube.Cube" true 0.5 null))
        (`PrimitiveComponent.AddImpulse` (`/Game/ThisProject/BP_Object.StaticMesh` _returnvalue) (0.0 0.0 100.0) "None" true)))))

(fn `UserConstructionScript`
  (`parent.UserConstructionScript`))