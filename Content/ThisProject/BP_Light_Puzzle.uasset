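; BP_Light_Puzzle is a color-mixing puzzle that spawns a golden crowbar item with a teleport effect once solved.
; Red, green and blue triggers set latched flags; the black trigger starts the puzzle, then checks them against the randomly chosen light color.
; Mixed colors require each component flag, and the flags are never cleared here.
; A failure resets the pass count and whitens the light; seven passes grant the one-time reward.
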(event `self.ReceiveBeginPlay`
  (`parent.ReceiveBeginPlay`)
  (add `/Game/ThisProject/Interactables/Switches/BP_WallButton.On Trigger` (`self.Red`) (`|CreateDelegate` :!event `Red Trigger`))
  (add `/Game/ThisProject/Interactables/Switches/BP_WallButton.On Trigger` (`self.Blue`) (`|CreateDelegate` :!event `Blue Trigger`))
  (add `/Game/ThisProject/Interactables/Switches/BP_WallButton.On Trigger` (`self.Green`) (`|CreateDelegate` :!event `Green Trigger`))
  (add `/Game/ThisProject/Interactables/Switches/BP_WallButton.On Trigger` (`self.Black`) (`|CreateDelegate` :!event `Black Trigger`)))

(event `Red Trigger`
  (set `self.R` true))

(event `Blue Trigger`
  (set `self.B` true))

(event `Green Trigger`
  (set `self.G` true))

(event `Black Trigger`
  (if (`self.Started`)
    (switch `int` (`self.Chosen Color`)
      (:`1`
        (if (`self.R`)
          (`self.Passed`)
          (else
            (`self.Fail` :!label _label))))
      (:`2`
        (if (`self.G`)
          (`self.Passed`)
          (else
            (goto _label))))
      (:`3`
        (if (`self.B`)
          (`self.Passed`)
          (else
            (goto _label))))
      (:`4`
        (if (`self.R`)
          (if (`self.G`)
            (`self.Passed`)
            (else
              (`self.Fail` :!label _label_2)))
          (else
            (goto _label_2))))
      (:`5`
        (if (`self.R`)
          (if (`self.B`)
            (`self.Passed`)
            (else
              (goto _label_2)))
          (else
            (goto _label_2))))
      (:`6`
        (if (`self.G`)
          (if (`self.B`)
            (`self.Passed`)
            (else
              (goto _label_2)))
          (else
            (goto _label_2))))
      (:`7`
        (if (`self.R`)
          (if (`self.G`)
            (if (`self.B`)
              (`self.Passed`)
              (else
                (goto _label_2)))
            (else
              (goto _label_2)))
          (else
            (goto _label_2)))))
    (else
      (`self.Change Light`)
      (set `self.Started` true))))

(event `Fail`
  (set `self.Started` false)
  (set `self.Passes` 0)
  (`self.Change Light Color` (struct :`R` 1.0 :`G` 1.0 :`B` 1.0 :`A` 1.0)))

(event `Change Light`
  (if (not (`self.Passed?`))
    (bind _output_get (set `self.Chosen Color` (`KismetMathLibrary.RandomIntegerInRange` 1 7)))
    (`self.Change Light Color` (select `int` _output_get :`0` (struct) :`1` (struct :`R` 1.0 :`A` 1.0) :`2` (struct :`G` 1.0 :`A` 1.0) :`3` (struct :`B` 1.0 :`A` 1.0) :`4` (struct :`R` 1.0 :`G` 1.0 :`A` 1.0) :`5` (struct :`R` 1.0 :`B` 1.0 :`A` 1.0) :`6` (struct :`G` 1.0 :`B` 1.0 :`A` 1.0) :`7` (struct :`R` 1.0 :`G` 1.0 :`B` 1.0 :`A` 1.0) :!type "LinearColor Structure"))))

(event `Passed`
  (bind _returnvalue (`SceneComponent.K2_GetComponentToWorld` (`self.Spawn`)))
  (bind _result (`/Engine/EditorBlueprintResources/StandardMacros.IncrementInt` (`self.Passes`))
    (:`  `
      (if (>= _result 7)
        (`/Engine/EditorBlueprintResources/StandardMacros.DoOnce` false
          (:`Completed`
            (`|SpawnActorFromClass` "/Game/ThisProject/Interactables/BP_Lootable_Item.BP_Lootable_Item_C" _returnvalue "Undefined" "MultiplyWithRoot" null (struct) (make `/Game/GridInventory/Data/ST_Item` "/Game/GridInventory/Data/DA_GoldenCrowBar_2.DA_GoldenCrowBar_2" 0.0 1) "/Engine/BasicShapes/Cube.Cube" true 0.5 null)
            (`NiagaraFunctionLibrary.SpawnSystemAtLocation` "/Game/ThisProject/Boss/NS_BossTeleport.NS_BossTeleport" (.location _returnvalue))
            (set `self.Passed?` true)
            (`self.Change Light Color` (struct :`R` 1.0 :`G` 1.0 :`B` 1.0 :`A` 1.0))))
        (else
          (`self.Change Light`))))))

(fn `UserConstructionScript`
  (`parent.UserConstructionScript`))