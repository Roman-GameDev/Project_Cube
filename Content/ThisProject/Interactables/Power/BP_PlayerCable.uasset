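; Interactable power cable that the player picks up, drops or plugs in to pass colored energy to an input.
; Interact toggles holding; a forward sphere trace snaps the end onto a hit component and sends it the Energy, and picking up again removes that power.
; A DoOnce-guarded drop turns the end into a physics object within cable length, also triggered by a looping distance check.
; The construction script tints cable and end from Energy gameplay tags.
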(event `Reset`
  (bind _returnvalue (`self.K2_GetActorLocation`))
  (bind _end (`self.End`))
  (bind _end_2 (`self.End`))
  (bind _returnvalue_2 (`SceneComponent.K2_GetComponentLocation` (`self.Parent`)))
  (`PrimitiveComponent.SetSimulatePhysics` (`self.End`) false)
  (`SceneComponent.K2_AttachToComponent` (`self.End`) (`self.Parent`) "None" "SnapToTarget" "SnapToTarget" "SnapToTarget" true)
  (goto _label :!via `Reset`))

(event `self.ReceiveBeginPlay`
  (`SceneComponent.K2_AttachToComponent` (`self.End`) (`self.Parent`) "None" "SnapToTarget" "SnapToTarget" "SnapToTarget" true)
  (`CableComponent.SetAttachEndToComponent` (`self.Cable`) (`self.End`) "None")
  (`KismetSystemLibrary.K2_SetTimerDelegate` (delegate `Check Distance`) 0.4 true))

(event `Drop`
  (bind _returnvalue (`self.K2_GetActorLocation`))
  (bind _end (`self.End`))
  (bind _end_2 (`self.End`))
  (bind _returnvalue_2 (`SceneComponent.K2_GetComponentLocation` (`self.Parent`)))
  (`/Engine/EditorBlueprintResources/StandardMacros.DoOnce` false :!label _label
    (:`Completed`
      (`SceneComponent.K2_DetachFromComponent` _end_2 "KeepWorld" "KeepWorld" "KeepWorld" true)
      (`CableComponent.SetAttachEndToComponent` (`self.Cable`) _end "None")
      (`SceneComponent.K2_SetWorldTransform` (`self.End`) (`KismetMathLibrary.MakeTransform` (`KismetMathLibrary.SelectVector` (+ _returnvalue (* (`KismetMathLibrary.GetDirectionUnitVector` _returnvalue _returnvalue_2) (- (`self.Cable Length`) 45.0))) _returnvalue_2 (> (`KismetMathLibrary.Vector_Distance` (`SceneComponent.K2_GetComponentLocation` (`self.Parent`)) (`SceneComponent.K2_GetComponentLocation` (`self.Cable`))) (`self.Cable Length`)))) false false)
      (`PrimitiveComponent.SetSimulatePhysics` _end_2 true)
      (`PrimitiveComponent.SetPhysicsLinearVelocity` _end (0.0 0.0 0.0) false "None"))))

(event `Check Distance`
  (if (> (`KismetMathLibrary.Vector_Distance` (`SceneComponent.K2_GetComponentLocation` (`self.Parent`)) (`SceneComponent.K2_GetComponentLocation` (`self.Cable`))) (`self.Cable Length`))
    (goto _label)))

(fn `Interact`
  (params (Interactor :type "Actor Object Reference") (`Interacting Component` :type "SceneComponent Object Reference"))
  (returns (Success :type Boolean))
  (if (`self.IsHeld`)
    (bind _success (`self.Trace For Plugs`))
    (if (not _success)
      (`self.Drop`)
      (set `self.IsHeld` false)
      (return false))
    (else
      (set `self.IsHeld` true)
      (`self.Reset`)
      (`CableComponent.SetAttachEndToComponent` (`self.Cable`) `Interacting Component` "None")
      (bind _connected_input (`self.Connected Input`)
        (:`then`
          (message `/Game/ThisProject/Interactables/Power/BPI_Power.Power Removed` _connected_input (`self.Energy`)))
        (:`else`
          _))
      (return false))))

(fn `Trace For Plugs`
  (returns (Success :type Boolean))
  (bind _end (`self.End`))
  (bind _parent (`self.Parent`))
  (bind _returnvalue (`SceneComponent.K2_GetComponentLocation` (`self.End`)))
  (bind (_outhit _returnvalue_2) (`KismetSystemLibrary.SphereTraceSingle` _returnvalue (+ _returnvalue (* (`KismetMathLibrary.Conv_RotatorToVector` (`KismetMathLibrary.ComposeRotators` (`SceneComponent.K2_GetComponentRotation` _parent) (* (`SceneComponent.RelativeRotation` _parent) -1.0))) 100.0)) 10.0 "TraceTypeQuery6"))
  (if _returnvalue_2
    (bind (_bblockinghit _binitialoverlap _time _distance _location _impactpoint _normal _impactnormal _physmat _hitactor _hitcomponent) (`GameplayStatics.BreakHitResult` _outhit))
    (`SceneComponent.K2_AttachToComponent` _end _hitcomponent "None" "SnapToTarget" "SnapToTarget" "SnapToTarget" true)
    (`CableComponent.SetAttachEndToComponent` (`self.Cable`) _end "None")
    (set `self.IsHeld` false)
    (`KismetSystemLibrary.K2_ClearTimer` null "Check Distance")
    (set `self.Connected Input` _hitcomponent)
    (message `/Game/ThisProject/Interactables/Power/BPI_Power.Power Energy` _hitcomponent (`self.Energy`))
    (return true)
    (else
      (return false))))

(fn `UserConstructionScript`
  (locals (`Last Cable End` :type "Transform Structure"))
  (`parent.UserConstructionScript`)
  (bind _returnvalue (`KismetMaterialLibrary.CreateDynamicMaterialInstance` "/Game/ThisProject/Rooms/Mat_Test_Red.Mat_Test_Red"))
  (`MaterialInstanceDynamic.SetVectorParameterValue` _returnvalue "color" (make `LinearColor` (`KismetMathLibrary.SelectFloat` 0.2 0.0 (`BlueprintGameplayTagLibrary.HasTag` (`self.Energy`) (struct :`TagName` "Energy.Red") true)) (`KismetMathLibrary.SelectFloat` 0.2 0.0 (`BlueprintGameplayTagLibrary.HasTag` (`self.Energy`) (struct :`TagName` "Energy.Green") true)) (`KismetMathLibrary.SelectFloat` 0.2 0.0 (`BlueprintGameplayTagLibrary.HasTag` (`self.Energy`) (struct :`TagName` "Energy.Blue") true)) 1.0))
  (`PrimitiveComponent.SetMaterial` (`self.Cable`) 0 _returnvalue)
  (`PrimitiveComponent.SetMaterial` (`self.End`) 0 _returnvalue))