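; BP_CableSpawn is an interactable power source that spawns player cables carrying its Energy gameplay tags.
; The construction script tints its static mesh through a dynamic material, mapping the red, green and blue Energy tags to color channels.
; Interact spawns a BP_PlayerCable at the Spawn component, passing Energy and the interacting component, then attaches it there.
; At MaxCables it destroys the last stored cable first, though CurrentCables only ever increments.
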(fn `Interact`
  (params (Interactor :type "Actor Object Reference") (`Interacting Component` :type "SceneComponent Object Reference"))
  (returns (Success :type Boolean))
  (bind _current_cables (`self.Current Cables`))
  (if (not (< _current_cables (`self.Max Cables`)))
    (bind _cable (`self.Cable`)
      (:`then`
        (`self.K2_DestroyActor` _cable))
      (:`else`
        _)))
  (`/Engine/EditorBlueprintResources/StandardMacros.IncrementInt` _current_cables
    (:`  `
      (bind _returnvalue (`|SpawnActorFromClass` "/Game/ThisProject/Interactables/Power/BP_PlayerCable.BP_PlayerCable_C" (`SceneComponent.K2_GetComponentToWorld` (`self.Spawn`)) "AlwaysSpawn" "MultiplyWithRoot" null `Interacting Component` (`self.Energy`) null))
      (set `self.Cable` _returnvalue)
      (`self.K2_AttachToComponent` _returnvalue (`self.Spawn`) "None" "SnapToTarget" "SnapToTarget" "SnapToTarget" true)
      (return false))))

(fn `UserConstructionScript`
  (`parent.UserConstructionScript`)
  (bind _returnvalue (`KismetMaterialLibrary.CreateDynamicMaterialInstance` "/Game/ThisProject/Rooms/Mat_Test_Red.Mat_Test_Red"))
  (`MaterialInstanceDynamic.SetVectorParameterValue` _returnvalue "color" (make `LinearColor` (`KismetMathLibrary.SelectFloat` 0.2 0.0 (`BlueprintGameplayTagLibrary.HasTag` (`self.Energy`) (struct :`TagName` "Energy.Red") true)) (`KismetMathLibrary.SelectFloat` 0.2 0.0 (`BlueprintGameplayTagLibrary.HasTag` (`self.Energy`) (struct :`TagName` "Energy.Green") true)) (`KismetMathLibrary.SelectFloat` 0.2 0.0 (`BlueprintGameplayTagLibrary.HasTag` (`self.Energy`) (struct :`TagName` "Energy.Blue") true)) 1.0))
  (`PrimitiveComponent.SetMaterial` (`self.StaticMesh`) 0 _returnvalue))