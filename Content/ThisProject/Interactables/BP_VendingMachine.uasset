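; Vending machine actor that offers purchasable items and dispenses them as lootable pickups.
; On BeginPlay it spawns and attaches a BP_Purchaseable_VendingItem button at each preset location, priced from a cost map; AddItem spawns a button for a new item.
; VendItems waits briefly, plays a sound and spawns a BP_Lootable_Item at the ItemSpawn point.
; Hacked triggers a one-time pass that calls VendItems for each HackableItems gameplay tag.
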(event `self.ReceiveBeginPlay`
  (bind _items_available (`self.Items Available`))
  (`parent.ReceiveBeginPlay`)
  (for (_array_element _array_index) (`self.Locations`)
    (bind _output (`|GetArrayItem` _items_available _array_index))
    (bind _returnvalue (`|SpawnActorFromClass` "/Game/ThisProject/Interactables/BP_Purchaseable_VendingItem.BP_Purchaseable_VendingItem_C" (`KismetMathLibrary.MakeTransform` (0.0 0.0 0.0)) "AlwaysSpawn" "MultiplyWithRoot" null (select `bool` (== (`KismetArrayLibrary.Array_Find` _items_available _output) -1) :`false` _output :`true` (struct :`TagName` "Items.Empty")) (`BlueprintMapLibrary.Map_Find` (`self.Items Cost Data`) _output) null))
    (`self.K2_AttachToActor` _returnvalue self "None" "SnapToTarget" "SnapToTarget" "SnapToTarget" true)
    (`self.K2_SetActorRelativeLocation` _returnvalue _array_element false false)
    (`KismetArrayLibrary.Array_Add` (`self.Buttons`) _returnvalue)))

(event `Hacked Vending Iterm`
  (`/Engine/EditorBlueprintResources/StandardMacros.DoOnce` false
    (:`Completed`
      (for _array_element (`BlueprintGameplayTagLibrary.BreakGameplayTagContainer` (`self.Hackable Items`))
        (`self.Vend Items` _array_element)))))

(event `/Game/ThisProject/Interactables/BPI_Vending.Vend Items`
  (params (Items :type "GameplayTag Structure") (Interactor :type "Actor Object Reference"))
  (`KismetSystemLibrary.Delay` 1.0)
  (`GameplayStatics.PlaySoundAtLocation` "/Game/ThisProject/SFX/MSS_VendItem.MSS_VendItem" (`self.K2_GetActorLocation`) (struct) 1.0 1.0 0.0 null null null null)
  (`|SpawnActorFromClass` "/Game/ThisProject/Interactables/BP_Lootable_Item.BP_Lootable_Item_C" (`SceneComponent.K2_GetComponentToWorld` (`self.Item Spawn`)) "AlwaysSpawn" "MultiplyWithRoot" null Items "/Engine/BasicShapes/Cube.Cube" true 1.0 null))

(event `/Game/ThisProject/Interactables/BPI_Vending.Add Item`
  (params (`New Item` :type "GameplayTag Structure"))
  (bind _items_available (`self.Items Available`))
  (bind _returnvalue (`KismetArrayLibrary.Array_Add` (`self.Items Available`) `New Item`))
  (`self.K2_DestroyActor` (`|GetArrayItem` (`self.Buttons`) _returnvalue))
  (bind _output (`|GetArrayItem` _items_available _returnvalue))
  (bind _returnvalue_2 (`|SpawnActorFromClass` "/Game/ThisProject/Interactables/BP_Purchaseable_VendingItem.BP_Purchaseable_VendingItem_C" (`KismetMathLibrary.MakeTransform` (0.0 0.0 0.0)) "AlwaysSpawn" "MultiplyWithRoot" null (select `bool` (== (`KismetArrayLibrary.Array_Find` _items_available _output) -1) :`false` _output :`true` (struct :`TagName` "Items.Empty")) (`BlueprintMapLibrary.Map_Find` (`self.Items Cost Data`) _output) null))
  (`self.K2_AttachToActor` _returnvalue_2 self "None" "SnapToTarget" "SnapToTarget" "SnapToTarget" true)
  (`self.K2_SetActorRelativeLocation` _returnvalue_2 (`|GetArrayItem` (`self.Locations`) _returnvalue) false false)
  (`KismetArrayLibrary.Array_Add` (`self.Buttons`) _returnvalue_2))

(fn `Hacked`
  (returns (Success :type Boolean))
  (`self.Hacked Vending Iterm`)
  (return true))

(fn `UserConstructionScript`
  (`parent.UserConstructionScript`))