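; BP_LootableWeapon is an interactable world pickup that hands a weapon to whoever interacts with it.
; The construction script sets the mesh from the Weapon variable's static mesh, so each instance displays its weapon.
; Trigger runs the parent logic, then sends LootWeaponMessage with the Weapon to the interactor.
; Interact runs the parent interaction, destroys the actor and returns the parent's result.
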(fn `Interact`
  (params (Interactor :type "Actor Object Reference") (`Interacting Component` :type "SceneComponent Object Reference"))
  (returns (Success :type Boolean))
  (bind _success (`parent.Interact` Interactor `Interacting Component`))
  (`self.K2_DestroyActor`)
  (return _success))

(fn `Trigger`
  (params (Interactor :type "Actor Object Reference"))
  (`parent.Trigger` Interactor)
  (message `/Game/ThisProject/Player/BPI_Interactor.Loot Weapon` Interactor (`self.Weapon`)))

(fn `UserConstructionScript`
  (`parent.UserConstructionScript`)
  (`StaticMeshComponent.SetStaticMesh` (`self.StaticMesh`) (`/Game/ThisProject/Player/DA_Weapon.Static Mesh` (`self.Weapon`))))