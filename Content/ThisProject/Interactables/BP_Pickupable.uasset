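; BP_Pickupable is an interactable physics prop that can be picked up and released.
; Interact disables mesh collision and physics, attaches to the interacting component and switches to first-person rendering.
; ClearInteraction detaches it, restores world rendering and re-enables collision and physics.
; Both call ReAttachActor to snap the mesh back onto the root, since physics simulation detaches it.
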(fn `Clear Interaction`
  (returns (Success :type Boolean))
  (bind _staticmesh (`self.StaticMesh`))
  (`PrimitiveComponent.SetFirstPersonPrimitiveType` (`self.StaticMesh`) "None")
  (`self.K2_DetachFromActor` "KeepWorld" "KeepWorld" "KeepWorld")
  (set `self.IsBeingHeld?` false)
  (`PrimitiveComponent.SetCollisionEnabled` _staticmesh "QueryAndPhysics")
  (`self.ReAttach Actor`)
  (`PrimitiveComponent.SetSimulatePhysics` _staticmesh true)
  (return true))

(fn `Interact`
  (params (Interactor :type "Actor Object Reference") (`Interacting Component` :type "SceneComponent Object Reference"))
  (returns (Success :type Boolean))
  (bind _staticmesh (`self.StaticMesh`))
  (if (not (`self.IsBeingHeld?`))
    (set `self.IsBeingHeld?` true)
    (`PrimitiveComponent.SetCollisionEnabled` _staticmesh "NoCollision")
    (`PrimitiveComponent.SetSimulatePhysics` _staticmesh false)
    (`SceneComponent.K2_SetWorldLocation` (`self.StaticMesh`) (+ (`SceneComponent.K2_GetComponentLocation` `Interacting Component`) (* (`SceneComponent.GetForwardVector` `Interacting Component`) 50.0) (0.0 0.0 35.0)) false false)
    (`self.ReAttach Actor`)
    (`self.K2_AttachToComponent` `Interacting Component` "None" "KeepWorld" "KeepWorld" "KeepWorld")
    (`PrimitiveComponent.SetFirstPersonPrimitiveType` _staticmesh "FirstPerson")
    (return true)))

(fn `ReAttach Actor`
  (`SceneComponent.K2_AttachToComponent` (`self.StaticMesh`) (`self.DefaultSceneRoot`) "None" "SnapToTarget" "SnapToTarget" "SnapToTarget" true))

(fn `UserConstructionScript`
  (`parent.UserConstructionScript`))