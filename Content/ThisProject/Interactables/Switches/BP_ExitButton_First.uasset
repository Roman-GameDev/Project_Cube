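; BP_ExitButton_First is a switch interactable, apparently the exit button for the first puzzle, that adds a voice-line cue to its parent's behavior.
; Its Trigger override runs the parent logic, then calls PlayDougLineMessage on the Game Instance with the Doug_FirstPuzzleDone line.
; All other events are disabled stubs, and the construction script only calls the parent.
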(event `self.Trigger`
  (`parent.Trigger`)
  (message `/Game/ThisProject/Player/BPI_GameInstance.Play Doug Line` (`GameplayStatics.GetGameInstance`) "/Game/ThisProject/Assets_Imports/Doug/Voicelines/Done/Doug_FirstPuzzleDone.Doug_FirstPuzzleDone"))

(fn `UserConstructionScript`
  (`parent.UserConstructionScript`))