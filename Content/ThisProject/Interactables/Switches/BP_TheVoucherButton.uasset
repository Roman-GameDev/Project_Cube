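; Interactable button that dispenses vouchers to whoever uses it, drawing from its own Vouchers counter.
; BeginPlay sets a timer by event, and a separate IncreaseVoucherCount event adds one to the counter.
; Interact takes one voucher when any remain and sends LootVouchers to the interactor, returning true even when the counter is empty.
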(event `self.ReceiveBeginPlay`
  (`parent.ReceiveBeginPlay`)
  (`KismetSystemLibrary.K2_SetTimerDelegate` (`|CreateDelegate` :!event `Increase Voucher Count`) 10.0))

(event `Increase Voucher Count`
  (`/Engine/EditorBlueprintResources/StandardMacros.IncrementInt` (`self.Vouchers`)))

(fn `Interact`
  (params (Interactor :type "Actor Object Reference") (`Interacting Component` :type "SceneComponent Object Reference"))
  (returns (Success :type Boolean))
  (if (> (`self.Vouchers`) 0)
    (`/Engine/EditorBlueprintResources/StandardMacros.DecrementInt` (`self.Vouchers`)
      (:`  `
        (message `/Game/ThisProject/Player/BPI_Interactor.Loot Vouchers` Interactor 1))))
  (return true))

(fn `UserConstructionScript`
  (`parent.UserConstructionScript`))