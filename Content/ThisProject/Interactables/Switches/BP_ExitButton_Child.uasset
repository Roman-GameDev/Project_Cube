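; BP_ExitButton_Child is an exit switch that runs the game's ending when triggered.
; Trigger calls the parent logic, sends the Game Instance a message to save hi-score values, then disables player input.
; It plays the LS_End level sequence with a stone-door choir sound, and after a delay adds the WB_EndScreen widget to the viewport.
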(event `self.Trigger`
  (bind _returnvalue (`GameplayStatics.GetPlayerController` 0))
  (`parent.Trigger`)
  (message `/Game/ThisProject/Player/BPI_GameInstance.Save Hi-Score Values` (`GameplayStatics.GetGameInstance`))
  (`self.DisableInput` _returnvalue _returnvalue)
  (bind (_outactor _returnvalue_2) (`LevelSequencePlayer.CreateLevelSequencePlayer` "/Game/ThisProject/Openinng/LS_End.LS_End"))
  (`MovieSceneSequencePlayer.Play` _returnvalue_2)
  (`GameplayStatics.PlaySound2D` "/Game/ThisProject/Openinng/581371__audiotorp__stonedoor_openswithchoir.581371__audiotorp__stonedoor_openswithchoir" 1.0 1.0 0.0 null null)
  (`KismetSystemLibrary.Delay` 8.0)
  (bind _returnvalue_3 (`|CreateWidget` "/Game/ThisProject/Openinng/WB_EndScreen.WB_EndScreen_C"))
  (`UserWidget.AddToViewport` _returnvalue_3 0))

(fn `UserConstructionScript`
  (`parent.UserConstructionScript`))