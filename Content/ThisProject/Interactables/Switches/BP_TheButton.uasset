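; BP_TheButton is an interactable switch that toggles a list of Triggerables on and off.
; Interact loops the movement of its DynamicStaticMesh, fires Trigger and returns true.
; Trigger uses a FlipFlop, so alternate presses send ActivateMessage or DeactivateMessage to every entry in Triggerables.
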(event `Trigger`
  (`/Engine/EditorBlueprintResources/StandardMacros.FlipFlop`
    (:`A`
      (for _array_element (`self.Triggerables`)
        (message `/Game/ThisProject/Interactables/Power/BPI_Activate.Activate` _array_element)))
    (:`B`
      (for _array_element_2 (`self.Triggerables`)
        (message `/Game/ThisProject/Interactables/Power/BPI_Activate.Deactivate` _array_element_2)))))

(fn `Interact`
  (params (Interactor :type "Actor Object Reference") (`Interacting Component` :type "SceneComponent Object Reference"))
  (returns (Success :type Boolean))
  (`/Game/ThisProject/Rooms/Dynamic_Static_Mesh.Loop Movement` (`self.Dynamic_Static_Mesh`))
  (`self.Trigger`)
  (return true))

(fn `UserConstructionScript`
  (`parent.UserConstructionScript`))