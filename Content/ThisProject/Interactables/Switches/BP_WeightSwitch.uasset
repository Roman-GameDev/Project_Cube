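; BP_WeightSwitch is a pressure switch that activates linked Triggerables while something overlaps its Box and deactivates them once the Box is empty.
; Toggling also drives DynamicStaticMesh to its end or start position, and Flip inverts the messages sent.
; With AutoGenerateConnectors set, BeginPlay traces down for the ground point and spawns a BP_Connector there for each Triggerable, with an End derived from that target's location.
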(event `self.ReceiveBeginPlay`
  (if (`self.Auto Generate Connectors`)
    (`self.Generate Connectors`)))

(event `/Game/ThisProject/Interactables/Switches/BPI_GenerateConnectors.Generate Connectors`
  (bind _returnvalue (`self.K2_GetActorLocation`))
  (bind _returnvalue_location (`KismetMathLibrary.BreakTransform` (`SceneComponent.K2_GetComponentToWorld` (`self.StaticMesh`))))
  (bind _outhit (`KismetSystemLibrary.LineTraceSingle` (+ _returnvalue (0.0 0.0 10.0)) (- _returnvalue (0.0 0.0 100.0)) "TraceTypeQuery1"))
  (for _array_element (`self.Triggerables`)
    (`|SpawnActorFromClass` "/Game/ThisProject/Interactables/Switches/BP_Connector.BP_Connector_C" (`KismetMathLibrary.MakeTransform` (`.Location` (`GameplayStatics.BreakHitResult` _outhit))) "Undefined" "MultiplyWithRoot" null (`KismetMathLibrary.InverseTransformLocation` (`KismetMathLibrary.MakeTransform` _returnvalue_location) (`self.K2_GetActorLocation` _array_element)) null)))

(event `self.Box.OnComponentBeginOverlap`
  (params (OverlappedComponent :type "PrimitiveComponent Object Reference") (OtherActor :type "Actor Object Reference") (OtherComp :type "PrimitiveComponent Object Reference") (OtherBodyIndex :type Integer) (bFromSweep :type Boolean) (SweepResult :type "HitResult Structure (by ref)"))
  (if (not (`self.IsToggled?`))
    (set `self.IsToggled?` true)
    (`/Game/ThisProject/Rooms/Dynamic_Static_Mesh.Force Move to End` (`self.Dynamic_Static_Mesh`))
    (if (`self.Flip`)
      (for _array_element (`self.Triggerables`) :!label _label
        (message `/Game/ThisProject/Interactables/Power/BPI_Activate.Deactivate` _array_element))
      (else
        (for _array_element_2 (`self.Triggerables`) :!label _label_2
          (message `/Game/ThisProject/Interactables/Power/BPI_Activate.Activate` _array_element_2))))))

(event `self.Box.OnComponentEndOverlap`
  (params (OverlappedComponent :type "PrimitiveComponent Object Reference") (OtherActor :type "Actor Object Reference") (OtherComp :type "PrimitiveComponent Object Reference") (OtherBodyIndex :type Integer))
  (if (`KismetArrayLibrary.Array_IsEmpty` (`PrimitiveComponent.GetOverlappingComponents` (`self.Box`)))
    (set `self.IsToggled?` false)
    (`/Game/ThisProject/Rooms/Dynamic_Static_Mesh.Force Move to Start` (`self.Dynamic_Static_Mesh`))
    (if (`self.Flip`)
      (goto _label_2)
      (else
        (goto _label)))))

(fn `UserConstructionScript`)