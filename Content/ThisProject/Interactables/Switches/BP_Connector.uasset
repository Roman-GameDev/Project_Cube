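; BP_Connector is a switch-related interactable piece that forms a thin, axis-aligned connecting line out to an End point.
; The construction script stretches and positions three segments (Root, Root1, Root2) from the End vector, chaining a Y run, an X run and a Z run with right-angle corners.
; It has no runtime logic, as the event graph holds only empty stub events.
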(fn `UserConstructionScript`
  (bind _end (`self.End`))
  (bind _end_2 (`self.End`))
  (bind _root1 (`self.Root1`))
  (`SceneComponent.SetRelativeScale3D` (`self.Root`) (`KismetMathLibrary.MakeVector` 0.1 (/ (.y (`self.End`)) 200.0) 0.01))
  (`SceneComponent.SetRelativeScale3D` _root1 (`KismetMathLibrary.MakeVector` (/ (.x _end_2) 100.0) 0.05 0.01))
  (`SceneComponent.K2_SetRelativeLocation` _root1 (`KismetMathLibrary.MakeVector` 5.0 (.y _end_2)) false false)
  (`SceneComponent.K2_SetRelativeLocation` (`self.Root2`) (`KismetMathLibrary.MakeVector` (.x _end) (.y _end)) false false)
  (`SceneComponent.SetRelativeScale3D` (`self.Root2`) (`KismetMathLibrary.MakeVector` 0.1 0.05 (/ (.z _end) 100.0))))