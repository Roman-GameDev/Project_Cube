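; BP_Terminal is an interactable terminal that plays a lore audio clip once.
; On BeginPlay it assigns an audio visualizer widget to its widget component.
; The first interaction destroys the decal, plays the MetaSound at the actor's location with the Lore wave passed as a parameter, and shows the widget.
; A Played flag and ignoring a custom trace channel on the mesh block further interaction.
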(event `self.ReceiveBeginPlay`
  (`parent.ReceiveBeginPlay`)
  (bind _returnvalue (`|CreateWidget` "/Game/ThisProject/Interactables/Terminal/WB_AudioVisualizer_Terminal.WB_AudioVisualizer_Terminal_C"))
  (`WidgetComponent.SetWidget` (`self.Widget`) _returnvalue))

(fn `Interact`
  (params (Interactor :type "Actor Object Reference") (`Interacting Component` :type "SceneComponent Object Reference"))
  (returns (Success :type Boolean))
  (if (not (`self.Played?`))
    (set `self.Played?` true)
    (`ActorComponent.K2_DestroyComponent` (`self.Decal`))
    (bind _returnvalue (`GameplayStatics.SpawnSoundAtLocation` "/Game/ThisProject/Interactables/Terminal/MSS_Terminal.MSS_Terminal" (`self.K2_GetActorLocation`) (struct) 1.0 1.0 0.0 null null))
    (`AudioComponent.SetWaveParameter` _returnvalue "sound" (`self.Lore`))
    (`AudioComponent.Play` _returnvalue 0.0)
    (`SceneComponent.SetVisibility` (`self.Widget`) true false)
    (`PrimitiveComponent.SetCollisionResponseToChannel` (`self.StaticMesh`) "ECC_GameTraceChannel3" "ECR_Ignore")
    (return true)))

(fn `UserConstructionScript`
  (`parent.UserConstructionScript`))