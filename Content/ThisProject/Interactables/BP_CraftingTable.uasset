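; BP_CraftingTable is an interactable crafting table that combines two golden crowbar parts from the interactor's inventory into a Golden Crowbar.
; Interact looks up both parts in the interactor's Comp_Inventory and, only when both are found, removes them and calls CraftCrowbar.
; CraftCrowbar plays a Niagara effect and spawns a physics-simulated BP_LootableWeapon carrying the crowbar data asset at the Spawn component.
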(event `Craft Crowbar`
  (params (Interactor :type "Actor Object Reference"))
  (bind _location (.location (`SceneComponent.K2_GetComponentToWorld` (`self.Spawn`))))
  (`NiagaraFunctionLibrary.SpawnSystemAtLocation` "/Game/ThisProject/Interactables/NS_Craft.NS_Craft" _location)
  (`|SpawnActorFromClass` "/Game/ThisProject/Interactables/BP_LootableWeapon.BP_LootableWeapon_C" (`KismetMathLibrary.MakeTransform` _location (.rotation (`SceneComponent.K2_GetComponentToWorld` (`self.Spawn`)))) "AlwaysSpawn" "MultiplyWithRoot" null "/Game/ThisProject/Player/DA_GoldenCrowbar.DA_GoldenCrowbar" "/Engine/BasicShapes/Cube.Cube" true 10.0 null))

(fn `Interact`
  (params (Interactor :type "Actor Object Reference") (`Interacting Component` :type "SceneComponent Object Reference"))
  (returns (Success :type Boolean))
  (bind _returnvalue (`self.GetComponentByClass` Interactor "/Game/GridInventory/Comp_Inventory.Comp_Inventory_C"))
  (bind (_success _key) (`/Game/GridInventory/Comp_Inventory.Find In Inventory` _returnvalue "/Game/GridInventory/Data/DA_GoldenCrowBar_1.DA_GoldenCrowBar_1"))
  (if _success
    (bind (_success_2 _key_2) (`/Game/GridInventory/Comp_Inventory.Find In Inventory` _returnvalue "/Game/GridInventory/Data/DA_GoldenCrowBar_2.DA_GoldenCrowBar_2"))
    (if _success_2
      (`/Game/GridInventory/Comp_Inventory.RemoveFromInventory` _returnvalue _key_2 true)
      (`/Game/GridInventory/Comp_Inventory.RemoveFromInventory` _returnvalue _key true)
      (`self.Craft Crowbar` Interactor)
      (return true))))

(fn `UserConstructionScript`
  (`parent.UserConstructionScript`))