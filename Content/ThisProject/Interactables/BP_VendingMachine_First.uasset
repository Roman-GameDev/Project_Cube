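; A scripted first vending machine whose first vend teleports the player to a replacement machine at a second location.
; It spawns that machine, offsets the player by the interactor's mirrored position using a floor trace, and rotates the view 180 degrees.
; It also destroys a designated machine, forwards the vend and attaches the spotlight to the replacement.
; Later vends use parent logic, and Activate adds a Svento item message to the replacement once.
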(event `self.ReceiveBeginPlay`
  (`parent.ReceiveBeginPlay`))

(event `/Game/ThisProject/Interactables/BPI_Vending.Vend Items`
  (params (Items :type "/Game/GridInventory/Data/DA_Items Object Reference") (Interactor :type "Actor Object Reference"))
  (bind _returnvalue (`GameplayStatics.GetPlayerController` 0))
  (bind _returnvalue_2 (`self.K2_GetActorLocation`))
  (bind _returnvalue_3 (`self.K2_GetActorLocation` Interactor))
  (bind _returnvalue_4 (`SceneComponent.K2_GetComponentToWorld` (`self.Second Vending Machine`)))
  (bind _returnvalue_5 (+ (.location _returnvalue_4) (* (`KismetMathLibrary.GetDirectionUnitVector` _returnvalue_3 _returnvalue_2) (`KismetMathLibrary.Vector_Distance` _returnvalue_2 _returnvalue_3))))
  (if (`self.Condition`)
    (`parent.Vend Items` Items Interactor)
    (else
      (set `self.Condition` true)
      (bind _returnvalue_6 (`|SpawnActorFromClass` "/Game/ThisProject/Interactables/BP_VendingMachine.BP_VendingMachine_C" _returnvalue_4 "AlwaysSpawn" "MultiplyWithRoot" null (struct) null (`|MakeArray` "/Game/GridInventory/Data/DA_Cigs.DA_Cigs" "/Game/GridInventory/Data/DA_SecondHeart.DA_SecondHeart" :!type "/Game/GridInventory/Data/DA_Items Object Reference") "/Game/ThisProject/Assets_Imports/Vending_Machine.Vending_Machine" false 3.0 null))
      (bind _outhit (`KismetSystemLibrary.LineTraceSingle` (+ _returnvalue_5 (0.0 0.0 100.0)) (- _returnvalue_5 (0.0 0.0 100.0)) "TraceTypeQuery1"))
      (`self.K2_SetActorLocation` (`GameplayStatics.GetPlayerCharacter` 0) (+ (`.Location` (`GameplayStatics.BreakHitResult` _outhit)) (0.0 0.0 20.0)) false false)
      (`self.K2_DestroyActor` (`self.Removed Vending Machine`))
      (`self.Vend Items` _returnvalue_6 Items Interactor)
      (`Controller.SetControlRotation` _returnvalue (`KismetMathLibrary.ComposeRotators` (`Controller.GetControlRotation` _returnvalue) (struct :`Yaw` 180.0)))
      (`SceneComponent.K2_AttachToComponent` (`self.SpotLight`) (`/Game/ThisProject/BP_Object.StaticMesh` _returnvalue_6) "None" "KeepRelative" "KeepRelative" "KeepRelative" true)
      (set `self.New VendingMachine` _returnvalue_6))))

(event `/Game/ThisProject/Interactables/Power/BPI_Activate.Activate`
  (`/Engine/EditorBlueprintResources/StandardMacros.DoOnce` false
    (:`Completed`
      (message `/Game/ThisProject/Interactables/BPI_Vending.Add Item` (`self.New VendingMachine`) "/Game/GridInventory/Data/DA_Svento.DA_Svento"))))

(fn `Check Activation`
  (returns (`Is Active` :type Boolean))
  (return false))

(fn `UserConstructionScript`
  (`parent.UserConstructionScript`))