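; BP_CableSpawn is an interactable that spawns a player cable when something interacts with it.
; Interact spawns a BP_PlayerCable at the StaticMesh's world transform, passing the interacting component as Parent and CableMaxLength as its length.
; The function always returns false, and the event graph and construction script add no logic of their own.
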(fn `Interact`
  (params (Interactor :type "Actor Object Reference") (`Interacting Component` :type "SceneComponent Object Reference"))
  (returns (Success :type Boolean))
  (`|SpawnActorFromClass` "/Game/ThisProject/Rooms/BP_PlayerCable.BP_PlayerCable_C" (`SceneComponent.K2_GetComponentToWorld` (`self.StaticMesh`)) "Undefined" "MultiplyWithRoot" null `Interacting Component` (`self.Cable Max Length`) null false null)
  (return false))

(fn `UserConstructionScript`
  (`parent.UserConstructionScript`))