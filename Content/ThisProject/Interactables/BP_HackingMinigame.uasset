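; Hacking minigame interactable where cables carrying energy feed power inputs to match a required RGB power pattern.
; On BeginPlay it creates power input components and spawns attached cable actors at configured locations.
; While powered, each energy change writes every input's RGB into a total map, overwriting rather than summing.
; If that map's values match the required ones, it sends HackedMessage to its linked actors.
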(event `self.ReceiveBeginPlay`
  (bind _returnvalue (`KismetMathLibrary.InvertTransform` (`self.GetTransform`)))
  (for (_array_element _array_index) (`self.Input Locations`)
    (bind _returnvalue_2 (`|AddComponentByClass` "/Game/ThisProject/Interactables/Power/SC_PowerInput.SC_PowerInput_C" false _array_element))
    (`/Game/ThisProject/Interactables/Power/SC_PowerInput.Initialize Power Input` _returnvalue_2 (`|GetArrayItem` (`self.Inputs`) _array_index))
    (`KismetArrayLibrary.Array_Add` (`self.Power`) (`/Game/ThisProject/Interactables/Power/SC_PowerInput.Comp_Power` _returnvalue_2))
    (add `/Game/ThisProject/Interactables/Power/SC_PowerInput.On Energy Change` _returnvalue_2 (`|CreateDelegate` :!event `Energy Changed`)))
  (for (_array_element_2 _array_index_2) (`self.Output Locations`)
    (bind _returnvalue_3 (`|SpawnActorFromClass` "/Game/ThisProject/Interactables/Power/BP_CableSpawn.BP_CableSpawn_C" (`KismetMathLibrary.MakeTransform` (`KismetMathLibrary.InverseTransformLocation` _returnvalue (.location _array_element_2)) (`KismetMathLibrary.InverseTransformRotation` _returnvalue (.rotation _array_element_2))) "AlwaysSpawn" "MultiplyWithRoot" null 50.0 (`|GetArrayItem` (`self.Outputs`) _array_index_2) 1 "/Game/Test/SM_TestCableEnd.SM_TestCableEnd" false null))
    (`self.K2_AttachToActor` _returnvalue_3 self "None" "KeepWorld" "KeepWorld" "KeepWorld" true)))

(event `Energy Changed`
  (bind _total_power (`self.Total Power`))
  (if (`self.IsPowered?`)
    (for _array_element (`self.Power`)
      (`BlueprintMapLibrary.Map_Add` _total_power "R" (`/Game/ThisProject/Comp_PowerRequired.R` _array_element))
      (`BlueprintMapLibrary.Map_Add` _total_power "G" (`/Game/ThisProject/Comp_PowerRequired.G` _array_element))
      (`BlueprintMapLibrary.Map_Add` _total_power "B" (`/Game/ThisProject/Comp_PowerRequired.B` _array_element)))
    (bind _values (`BlueprintMapLibrary.Map_Values` (`self.Total Power`)))
    (bind _values_2 (`BlueprintMapLibrary.Map_Values` (`self.Required Power`)))
    (if (`KismetArrayLibrary.Array_Identical` _values _values_2)
      (for _array_element_2 (`self.HackedActors`)
        (message `/Game/ThisProject/Interactables/BPI_Hack.Hacked` _array_element_2)))))

(event `/Game/ThisProject/Interactables/Power/BPI_Power.Power SIgnal`
  (params (`Powered?` :type Boolean))
  (set `self.IsPowered?` `Powered?`))

(fn `Change Energy`
  (params (Value :type "Integer (by ref)") (Key :type String) (Index :type Integer))
  (bind _total_power (`self.Total Power`))
  (`BlueprintMapLibrary.Map_Add` _total_power Key (+ 0 (`BlueprintMapLibrary.Map_Find` _total_power Key))))

(fn `UserConstructionScript`)