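; Interactable door that opens and closes through a door component, with Trigger and Untrigger events gated by power.
; A power input component, initialized with the required energy tags at construction, sets the powered flag through its on/off events.
; The Power Check macro blocks triggering only when Energy.Blue is required and power is off.
; Direct Open and Close calls skip the check, as does the construction script setting the initial state.
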(event `Open`
  (`/Game/ThisProject/Rooms/SC_Door.Open Door` (`self.SC_Door`)))

(event `Close`
  (`/Game/ThisProject/Rooms/SC_Door.Close Door` (`self.SC_Door`)))

(event `self.Trigger`
  (`self.Power Check`)
  (`self.Open`))

(event `self.Untrigger`
  (`self.Power Check`)
  (`self.Close`))

(event `self.SC_PowerInput.On Power On`
  (set `self.IsPowered?` true))

(event `self.SC_PowerInput.On Power Off`
  (set `self.IsPowered?` false))

(fn `UserConstructionScript`
  (`parent.UserConstructionScript`)
  (`/Game/ThisProject/Interactables/Power/SC_PowerInput.Initialize Power Input` (`self.SC_PowerInput`) (`self.Required Energy`))
  (if (`self.Start Open?`)
    (`self.Open`)
    (else
      (`self.Close`))))