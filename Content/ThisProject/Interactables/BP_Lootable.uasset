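; BP_Lootable is an interactable actor that acts as a one-shot pickup, removed from the world once used.
; Interact passes the interactor to Trigger, destroys the actor and returns true.
; Trigger is empty here, serving as a hook for the loot effect, and the event graph holds only disabled default events.
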(fn `Interact`
  (params (Interactor :type "Actor Object Reference") (`Interacting Component` :type "SceneComponent Object Reference"))
  (returns (Success :type Boolean))
  (`self.Trigger` Interactor)
  (`self.K2_DestroyActor`)
  (return true))

(fn `Trigger`
  (params (Interactor :type "Actor Object Reference")))

(fn `UserConstructionScript`
  (`parent.UserConstructionScript`))