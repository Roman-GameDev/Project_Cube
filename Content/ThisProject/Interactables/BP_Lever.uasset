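; BP_Lever is an interactable two-position lever that switches two sets of linked triggerables in opposition.
; Each Interact call runs a FlipFlop that forces the DynamicStaticMesh to its end or start.
; At the end, ForwardTriggerables receive activate messages and BackwardTriggerables deactivate; at the start, the reverse.
; BeginPlay applies the start state by entering that branch directly, bypassing the FlipFlop, so the first interaction moves forward.
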(event `self.ReceiveBeginPlay`
  (`parent.ReceiveBeginPlay`)
  (`self.Start`))

(event `Flip`
  (`/Engine/EditorBlueprintResources/StandardMacros.FlipFlop`
    (:`A`
      (`/Game/ThisProject/Rooms/Dynamic_Static_Mesh.Force Move to End` (`self.Dynamic_Static_Mesh`))
      (for _array_element (`self.Forward Triggerables`)
        (message `/Game/ThisProject/Interactables/Power/BPI_Activate.Activate` _array_element))
      (for _array_element_2 (`self.Backward Triggerables`)
        (message `/Game/ThisProject/Interactables/Power/BPI_Activate.Deactivate` _array_element_2)))
    (:`B`
      (`/Game/ThisProject/Rooms/Dynamic_Static_Mesh.Force Move to Start` (`self.Dynamic_Static_Mesh`) :!label _label)
      (for _array_element_3 (`self.Backward Triggerables`)
        (message `/Game/ThisProject/Interactables/Power/BPI_Activate.Activate` _array_element_3))
      (for _array_element_4 (`self.Forward Triggerables`)
        (message `/Game/ThisProject/Interactables/Power/BPI_Activate.Deactivate` _array_element_4)))))

(event `Start`
  (goto _label))

(fn `Interact`
  (params (Interactor :type "Actor Object Reference") (`Interacting Component` :type "SceneComponent Object Reference"))
  (returns (Success :type Boolean))
  (`self.Flip`)
  (return false))

(fn `UserConstructionScript`
  (`parent.UserConstructionScript`))