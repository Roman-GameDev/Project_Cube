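; BP_Platform is a powerable interactable platform that moves between two positions when activated or deactivated.
; Activation forces its DynamicStaticMesh to the end position, and deactivation forces it back to the start.
; Each change plays the matching door open or close sound at the actor's location with a raised pitch.
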(event `self.ReceiveBeginPlay`
  (`parent.ReceiveBeginPlay`))

(event `self.Activate Powerable`
  (`/Game/ThisProject/Rooms/Dynamic_Static_Mesh.Force Move to End` (`self.Dynamic_Static_Mesh`))
  (`GameplayStatics.PlaySoundAtLocation` "/Game/ThisProject/SFX/MSS_DoorOpen.MSS_DoorOpen" (`self.K2_GetActorLocation`) (struct) 1.0 4.0 0.0 null null null null))

(event `self.Deactivate Powerable`
  (`/Game/ThisProject/Rooms/Dynamic_Static_Mesh.Force Move to Start` (`self.Dynamic_Static_Mesh`))
  (`GameplayStatics.PlaySoundAtLocation` "/Game/ThisProject/SFX/MSS_DoorClose.MSS_DoorClose" (`self.K2_GetActorLocation`) (struct) 1.0 4.0 0.0 null null null null))

(fn `UserConstructionScript`
  (`parent.UserConstructionScript`))