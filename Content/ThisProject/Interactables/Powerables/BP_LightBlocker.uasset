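; BP_LightBlocker is a powerable interactable that shifts a dynamic static mesh between two end positions, presumably to block light.
; Activating forces the mesh to its end with a door-open sound, and deactivating returns it to the start with a door-close sound, both high-pitched.
; A Flip flag swaps the two responses, so power can drive the mesh in either direction.
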(event `self.ReceiveBeginPlay`
  (`parent.ReceiveBeginPlay`))

(event `self.Activate Powerable`
  (bind _returnvalue (`self.K2_GetActorLocation`))
  (bind _dynamic_static_mesh (`self.Dynamic_Static_Mesh`))
  (if (`self.Flip?`)
    (`/Game/ThisProject/Rooms/Dynamic_Static_Mesh.Force Move to Start` _dynamic_static_mesh :!label _label)
    (`GameplayStatics.PlaySoundAtLocation` "/Game/ThisProject/SFX/MSS_DoorClose.MSS_DoorClose" _returnvalue (struct) 1.0 4.0 0.0 null null null null)
    (else
      (`/Game/ThisProject/Rooms/Dynamic_Static_Mesh.Force Move to End` _dynamic_static_mesh :!label _label_2)
      (`GameplayStatics.PlaySoundAtLocation` "/Game/ThisProject/SFX/MSS_DoorOpen.MSS_DoorOpen" _returnvalue (struct) 1.0 4.0 0.0 null null null null))))

(event `self.Deactivate Powerable`
  (if (`self.Flip?`)
    (goto _label_2)
    (else
      (goto _label))))

(fn `UserConstructionScript`
  (`parent.UserConstructionScript`))