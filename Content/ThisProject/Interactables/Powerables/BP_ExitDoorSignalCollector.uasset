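; Exit door signal collector that shows how many signals have been collected through a set of four decals.
; The construction script stores the decals in an array in the order 0, 3, 2, 1.
; Each SignalCollected event uses the Collected count to pick the next decal and sets its alpha to full, copying the RGB color from the first decal.
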(event `self.Signal Collected`
  (bind (_r _g _b) (`KismetMathLibrary.BreakColor` (`DecalComponent.DecalColor` (`self.Decal_0`))))
  (`DecalComponent.SetDecalColor` (`|GetArrayItem` (`self.Array of Decals`) (- (`self.Collected`) 1)) (make `LinearColor` _r _g _b 1.0)))

(fn `UserConstructionScript`
  (`parent.UserConstructionScript`)
  (set `self.Array of Decals` (`|MakeArray` (`self.Decal_0`) (`self.Decal3`) (`self.Decal2`) (`self.Decal1`))))