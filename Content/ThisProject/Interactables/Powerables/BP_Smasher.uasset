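; BP_Smasher is a powerable environmental hazard that cycles between active and inactive states and damages what it hits.
; It activates on BeginPlay and starts a looping SmashTime timer, with a Smash FlipFlop alternating Deactivate and Activate.
; Deactivate starts a timer matching the DynamicStaticMesh's Time, apparently delaying damage until the movement ends.
; Damage box-traces at the Arrow and sends each hit actor an Environment-tagged ApplyDamage message.
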(event `self.ReceiveBeginPlay`
  (`parent.ReceiveBeginPlay`)
  (`self.Activate`)
  (`KismetSystemLibrary.K2_SetTimerDelegate` (`|CreateDelegate` :!event `Smash`) (`self.Smash Time`) true))

(event `Smash`
  (`/Engine/EditorBlueprintResources/StandardMacros.FlipFlop`
    (:`A`
      (`self.Deactivate`))
    (:`B`
      (`self.Activate`))))

(event `/Game/ThisProject/Interactables/Power/BPI_Activate.Deactivate`
  (`parent.Deactivate`)
  (`KismetSystemLibrary.K2_SetTimerDelegate` (`|CreateDelegate` :!event `Damage`) (`/Game/ThisProject/Rooms/Dynamic_Static_Mesh.Time` (`self.Dynamic_Static_Mesh`))))

(event `Damage`
  (bind _returnvalue (`SceneComponent.K2_GetComponentLocation` (`self.Arrow`)))
  (bind _outhits (`KismetSystemLibrary.BoxTraceMulti` _returnvalue (- _returnvalue (0.0 0.0 1.0)) (28.0 32.0 150.0) (struct) "TraceTypeQuery1"))
  (for _array_element _outhits
    (message `/Game/ThisProject/BPI_Health.Apply Damage` (`.HitActor` (`GameplayStatics.BreakHitResult` _array_element)) (make `/Game/ThisProject/Struct_DamageHitResult` 10.0 _array_element (struct :`GameplayTags` (struct :`(TagName` "DamageSource.Environment")))))))

(fn `UserConstructionScript`
  (`parent.UserConstructionScript`))