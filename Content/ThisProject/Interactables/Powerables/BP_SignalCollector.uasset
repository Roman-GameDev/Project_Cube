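; BP_SignalCollector is a powerable interactable that counts incoming signals and spawns an exit button once enough arrive.
; Each Activate increments Collected and fires the empty SignalCollected event.
; At four or more, it spawns BP_ExitButton_Child at SpawnLocaiton, passing on its Triggerables and a podium mesh; further activations spawn again.
; A loop messaging Triggerables directly is left unconnected.
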(event `/Game/ThisProject/Interactables/Power/BPI_Activate.Activate`
  (bind _result (`/Engine/EditorBlueprintResources/StandardMacros.IncrementInt` (`self.Collected`))
    (:`  `
      (`self.Signal Collected`)
      (if (>= _result 4)
        (`|SpawnActorFromClass` "/Game/ThisProject/Interactables/Switches/BP_ExitButton_Child.BP_ExitButton_Child_C" (`SceneComponent.K2_GetComponentToWorld` (`self.Spawn Locaiton`)) "AlwaysSpawn" "MultiplyWithRoot" null (`self.Triggerables`) true "/Game/ThisProject/Assets_Imports/Button_Podium.Button_Podium" false 3.0 null)))))

(event `Signal Collected`)

(fn `UserConstructionScript`
  (`parent.UserConstructionScript`))