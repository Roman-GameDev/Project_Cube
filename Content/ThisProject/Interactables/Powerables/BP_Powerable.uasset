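; Base powerable interactable with empty ActivatePowerable and DeactivatePowerable events as hooks for behavior.
; If RequiredEnergy matches Energy.Blue, it spawns an SC_PowerInput and binds its power events; otherwise it becomes trigger-only with a default orange overlay.
; PowerOn and PowerOff call Activate or Deactivate unless RequiresTrigger, before updating IsPowered, which gates both hooks when power is required.
; A dynamic overlay material shows current energy by mapping Red, Green and Blue tags to color channels.
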(event `self.ReceiveBeginPlay`
  (`|ExecutionSequence`
    (:`then_0`
      (bind _returnvalue (`KismetMaterialLibrary.CreateDynamicMaterialInstance` "/Game/ThisProject/Interactables/Powerables/Mat_PowerOutline_Inst.Mat_PowerOutline_Inst"))
      (set `self.Power Overlay` _returnvalue)
      (`MeshComponent.SetOverlayMaterial` (`self.GetComponentByClass` "/Script/Engine.StaticMeshComponent") (`self.Power Overlay`))
      (bind _output_get (set `self.Requires Power?` (`BlueprintGameplayTagLibrary.HasAnyTags` (`self.Required Energy`) (`BlueprintGameplayTagLibrary.MakeLiteralGameplayTagContainer` (struct :`GameplayTags` (struct :`(TagName` "Energy.Blue") :`(TagName` "Energy.Green") :`(TagName` "Energy.Red")))))))
      (if _output_get
        (bind _returnvalue_2 (`|AddComponentByClass` "/Game/ThisProject/Interactables/Power/SC_PowerInput.SC_PowerInput_C" false (`SceneComponent.GetRelativeTransform` (`self.Power Input Location`)) (`self.Required Energy`)))
        (add `/Game/ThisProject/Interactables/Power/SC_PowerInput.On Power On` _returnvalue_2 (`|CreateDelegate` :!event `Power On`))
        (add `/Game/ThisProject/Interactables/Power/SC_PowerInput.On Power Off` _returnvalue_2 (`|CreateDelegate` :!event `Power Off`))
        (set `self.Power Input` _returnvalue_2)
        (else
          (set `self.Requires Trigger?` true)
          (`self.Change Power Color Default`))))))

(event `Power On`
  (if (not (`self.Requires Trigger?`))
    (`self.Activate`))
  (set `self.IsPowered?` true)
  (`self.Change Power Color`))

(event `Power Off`
  (if (not (`self.Requires Trigger?`))
    (`self.Deactivate`))
  (set `self.IsPowered?` false)
  (`self.Change Power Color`))

(event `/Game/ThisProject/Interactables/Power/BPI_Activate.Deactivate`
  (if (`self.Requires Power?`)
    (if (`self.IsPowered?`)
      (`self.Deactivate Powerable` :!label _label))
    (else
      (goto _label))))

(event `Change Power Color Default`
  (`MaterialInstanceDynamic.SetVectorParameterValue` (`self.Power Overlay`) "color" (struct :`R` 1.0 :`G` 0.25 :`A` 1.0)))

(event `/Game/ThisProject/Interactables/Power/BPI_Activate.Activate`
  (if (`self.Requires Power?`)
    (if (`self.IsPowered?`)
      (`self.Activate Powerable` :!label _label_2))
    (else
      (goto _label_2))))

(event `Change Power Color`
  (bind _current_energy (`/Game/ThisProject/Interactables/Power/Comp_PowerRequired.Current Energy` (`/Game/ThisProject/Interactables/Power/SC_PowerInput.Comp_Power` (`self.Power Input`))))
  (`MaterialInstanceDynamic.SetVectorParameterValue` (`self.Power Overlay`) "color" (`KismetMathLibrary.MakeColor` (`KismetMathLibrary.SelectFloat` 1.0 0.0 (`BlueprintGameplayTagLibrary.HasTag` _current_energy (struct :`TagName` "Energy.Red"))) (`KismetMathLibrary.SelectFloat` 1.0 0.0 (`BlueprintGameplayTagLibrary.HasTag` _current_energy (struct :`TagName` "Energy.Green"))) (`KismetMathLibrary.SelectFloat` 1.0 0.0 (`BlueprintGameplayTagLibrary.HasTag` _current_energy (struct :`TagName` "Energy.Blue"))))))

(event `Activate Powerable`)

(event `Deactivate Powerable`)

(fn `UserConstructionScript`)