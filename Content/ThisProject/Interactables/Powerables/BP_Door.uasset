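; BP_Door is a powerable door that opens when powered and closes when power is removed, playing a sound at its location each time.
; Its activate and deactivate events drive the SCDoor component's open and close calls.
; On BeginPlay it gives the door mesh's second material slot a dynamic light material tinted with the required power color.
; The construction script shows or hides a spotlight from the ActivateLight setting.
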(event `self.ReceiveBeginPlay`
  (`parent.ReceiveBeginPlay`)
  (bind _returnvalue (`KismetMaterialLibrary.CreateDynamicMaterialInstance` "/Game/ThisProject/Materials/Mat_DoorLight.Mat_DoorLight"))
  (`MaterialInstanceDynamic.SetVectorParameterValue` _returnvalue "Light Color" (`self.Get Power Required Color`))
  (`PrimitiveComponent.SetMaterial` (`self.SC_Door`) 1 _returnvalue))

(event `self.ReceiveActorBeginOverlap`
  (params (OtherActor :type "Actor Object Reference"))
  (`parent.ReceiveActorBeginOverlap` OtherActor))

(event `self.Activate Powerable`
  (`/Game/ThisProject/Rooms/SC_Door.Open Door` (`self.SC_Door`))
  (`GameplayStatics.PlaySoundAtLocation` "/Game/ThisProject/SFX/MSS_DoorOpen.MSS_DoorOpen" (`self.K2_GetActorLocation`) (struct) 1.0 1.0 0.0 null null null null))

(event `self.Deactivate Powerable`
  (`/Game/ThisProject/Rooms/SC_Door.Close Door` (`self.SC_Door`))
  (`GameplayStatics.PlaySoundAtLocation` "/Game/ThisProject/SFX/MSS_DoorClose.MSS_DoorClose" (`self.K2_GetActorLocation`) (struct) 1.0 1.0 0.0 null null null null))

(fn `UserConstructionScript`
  (`parent.UserConstructionScript`)
  (`SceneComponent.SetVisibility` (`self.SpotLight`) (`self.Activate Light?`) false))