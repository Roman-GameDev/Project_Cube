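; BP_Lootable_Item is an interactable world pickup for a single item, described by its ItemData struct.
; The construction script sets the static mesh and any valid materials from that item data.
; When triggered, it passes itself and its item data to the interactor through PickUpItemMessage and destroys itself if the pickup succeeds.
; ModifyQuantity overwrites the stored quantity and always returns false.
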(fn `Modify Quantity`
  (params (Quantity :type Integer))
  (returns (Return :type Boolean))
  (setmembers `/Game/GridInventory/Data/ST_Item` :`StructRef` (`self.Item Data`) :`Quantity` Quantity)
  (return false))

(fn `Trigger`
  (params (Interactor :type "Actor Object Reference"))
  (`parent.Trigger` Interactor)
  (bind _return (message `/Game/ThisProject/Player/BPI_Interactor.Pick Up Item` Interactor self (`self.Item Data`)))
  (if _return
    (`self.K2_DestroyActor`)))

(fn `UserConstructionScript`
  (bind _staticmesh (`self.StaticMesh`))
  (bind ((`Data_2_F3A1C4BF456F492026C721B9BCBE8DF0` _data)) (break `/Game/GridInventory/Data/ST_Item` (`self.Item Data`)))
  (`parent.UserConstructionScript`)
  (`StaticMeshComponent.SetStaticMesh` _staticmesh (`/Game/GridInventory/Data/DA_Items.Static Mesh` _data))
  (for (_array_element _array_index) (`/Game/GridInventory/Data/DA_Items.Materials` _data)
    (`/Engine/EditorBlueprintResources/StandardMacros.IsValid` _array_element
      (:`Is Valid`
        (`PrimitiveComponent.SetMaterial` _staticmesh _array_index _array_element)))))