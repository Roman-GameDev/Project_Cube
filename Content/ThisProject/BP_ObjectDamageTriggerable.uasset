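; BP_ObjectDamageTriggerable is a base Blueprint for an object that fires a trigger whenever damage is applied to it.
; Its Apply Damage override runs the parent logic, passes the damage info to the Trigger event, then always returns false.
; Trigger is an empty hook here, and the construction script only calls the parent.
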(event `Trigger`
  (params (Damage :type "/Game/ThisProject/Struct_DamageHitResult Structure")))

(fn `Apply Damage`
  (params (`Damage Info` :type "/Game/ThisProject/Struct_DamageHitResult Structure"))
  (returns (Success :type Boolean))
  (`parent.Apply Damage` `Damage Info`)
  (`self.Trigger` `Damage Info`)
  (return false))

(fn `UserConstructionScript`
  (`parent.UserConstructionScript`))