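; BP_PortablePort is an actor that spawns cable connection points on those of its ports tagged for Energy.
; The construction script builds an ordered array of six directional port components: top, bottom and the X and Y sides.
; On BeginPlay it walks the Ports map values and spawns a BP_CableSpawn for each Energy match, passing its tags and snapping it to the component at the same index.
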(event `self.ReceiveBeginPlay`
  (`parent.ReceiveBeginPlay`)
  (bind _values (`BlueprintMapLibrary.Map_Values` (`self.Ports`)))
  (for (_array_element _array_index) _values
    (if (`BlueprintGameplayTagLibrary.HasAnyTags` _array_element (`BlueprintGameplayTagLibrary.MakeLiteralGameplayTagContainer` (struct :`GameplayTags` (struct :`(TagName` "Energy")))))
      (bind _returnvalue (`|SpawnActorFromClass` :`Class` "/Game/ThisProject/Interactables/Power/BP_CableSpawn.BP_CableSpawn_C" :`SpawnTransform` (`KismetMathLibrary.MakeTransform` (0.0 0.0 0.0)) :`CollisionHandlingOverride` "AlwaysSpawn" :`TransformScaleMethod` "MultiplyWithRoot" :`Energy` _array_element :`Show Decal?` false :`Mesh` "/Game/Test/SM_TestCableEnd.SM_TestCableEnd" :`Instigator` null))
      (`self.K2_AttachToComponent` _returnvalue (`|GetArrayItem` (`self.Ports Comp`) _array_index) "None" "SnapToTarget" "SnapToTarget" "SnapToTarget" true))))

(fn `UserConstructionScript`
  (`parent.UserConstructionScript`)
  (set `self.Ports Comp` (`|MakeArray` (`self.Top`) (`self.Bottom`) (`self.X`) (`self.-X`) (`self.Y`) (`self.-Y`) :!type "SceneComponent Object Reference")))