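; BP_DeadBody is a headless enemy corpse prop that the player can loot once.
; On BeginPlay it hides the head bone and turns on physics simulation from both thigh bones down.
; Its Interact function, on first use, sends the interactor a voucher pack item message by gameplay tag and makes the budgeted skeletal mesh ignore a trace channel.
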(event `self.ReceiveBeginPlay`
  (bind _skeletalmeshcomponentbudgeted (`self.SkeletalMeshComponentBudgeted`))
  (`SkinnedMeshComponent.HideBoneByName` _skeletalmeshcomponentbudgeted "head" "PBO_None")
  (`SkeletalMeshComponent.SetAllBodiesBelowSimulatePhysics` _skeletalmeshcomponentbudgeted "Thigh_R" true true)
  (`SkeletalMeshComponent.SetAllBodiesBelowSimulatePhysics` _skeletalmeshcomponentbudgeted "Thigh_L" true true))

(fn `Clear Interaction`
  (returns (Success :type Boolean))
  (return false))

(fn `Interact`
  (params (Interactor :type "Actor Object Reference") (`Interacting Component` :type "SceneComponent Object Reference"))
  (returns (Success :type Boolean))
  (if (not (`self.Looted`))
    (set `self.Looted` true)
    (message `/Game/ThisProject/Player/BPI_Interactor.Use Item` Interactor (`BlueprintGameplayTagLibrary.MakeLiteralGameplayTag` (struct :`TagName` "Items.VoucherPack.10")))
    (`PrimitiveComponent.SetCollisionResponseToChannel` (`self.SkeletalMeshComponentBudgeted`) "ECC_GameTraceChannel3" "ECR_Ignore")
    (return true)))

(fn `UserConstructionScript`)