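; BP_Object is a configurable world object with a static mesh, optional physics, optional sound and health.
; The construction script applies the exposed mesh and physics settings and makes the mesh block a custom game trace channel.
; BeginPlay attaches the sound, if set, and scales the mesh's mass.
; ApplyDamage forwards damage info to the CompHealth component and always returns false.
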(event `self.ReceiveBeginPlay`
  (bind _sound (`self.Sound`)
    (:`then`
      (`GameplayStatics.SpawnSoundAttached` _sound (`self.StaticMesh`) "None" (0.0 0.0 0.0) (struct) "KeepRelativeOffset" false 1.0 1.0 0.0 null null))
    (:`else`
      _))
  (`PrimitiveComponent.SetAllMassScale` (`self.StaticMesh`) (`self.Mass`)))

(fn `Apply Damage`
  (params (`Damage Info` :type "/Game/ThisProject/Struct_DamageHitResult Structure"))
  (returns (Success :type Boolean))
  (`/Game/ThisProject/Comp_Health.Apply Damage to Health` (`self.Comp_Health`) `Damage Info`)
  (return false))

(fn `UserConstructionScript`
  (bind _staticmesh (`self.StaticMesh`))
  (`parent.UserConstructionScript`)
  (`StaticMeshComponent.SetStaticMesh` _staticmesh (`self.Mesh`))
  (`PrimitiveComponent.SetSimulatePhysics` _staticmesh (`self.Simulate Physics`))
  (`PrimitiveComponent.SetCollisionResponseToChannel` (`self.StaticMesh`) "ECC_GameTraceChannel3" "ECR_Block"))