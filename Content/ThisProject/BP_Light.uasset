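; BP_Light is a light actor with a spotlight that can flicker, controlled by a Flicker flag checked at BeginPlay.
; When enabled, a timer chain switches the SpotLight intensity to zero, restores it to a fixed brightness shortly after, and schedules the next blink after a random delay.
; The effect runs entirely on timers, with Tick left disabled.
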(event `self.ReceiveBeginPlay`
  (`parent.ReceiveBeginPlay`)
  (if (`self.Flicker?`)
    (`KismetSystemLibrary.K2_SetTimerDelegate` (`|CreateDelegate` :!event `Flicker`) 0.1)))

(event `Flicker`
  (`LightComponent.SetIntensity` (`self.SpotLight`) 0.0)
  (`KismetSystemLibrary.K2_SetTimerDelegate` (delegate `Reset Flicker`) 0.1)
  (`KismetSystemLibrary.K2_SetTimerDelegate` (delegate `Flicker`) (`KismetMathLibrary.RandomFloatInRange` 0.4 1.0)))

(event `Reset Flicker`
  (`LightComponent.SetIntensity` (`self.SpotLight`) 3000.0))

(fn `UserConstructionScript`
  (`parent.UserConstructionScript`))