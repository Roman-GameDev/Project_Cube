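; Boss actor that runs a timed arena fight with music and a health bar, then explodes and messages a door on death.
; Looping timers drive an accelerating, line-traced machine-gun barrage and cultist spawns behind the player.
; Proximity or height checks teleport it between preset points, while a spinning shell animates it between attacks.
; Non-explosive damage is quartered; heavy hits stun it with physics simulation until it resets.
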(event `Spawn`
  ; Spawn Enemies
  (for _ (range 1 (+ (`KismetMathLibrary.RandomIntegerInRange` 1 3) 1))
    (`self.Spawn Minions`)))

(event `Spawn Minions`
  (bind _target (`self.Target`))
  (bind _arena (`self.Arena`))
  (bind _returnvalue (+ (`self.K2_GetActorLocation` _target) (* (`SceneComponent.GetForwardVector` (`Character.Mesh` _target)) -500.0)))
  ; Spawn Enemies
  (if (`KismetMathLibrary.IsPointInBox` _returnvalue (`SceneComponent.K2_GetComponentLocation` _arena) (`BoxComponent.BoxExtent` _arena))
    (bind (_outhit _returnvalue_2) (`KismetSystemLibrary.LineTraceSingle` (+ _returnvalue (0.0 0.0 100.0)) (- _returnvalue (0.0 0.0 1000.0)) "TraceTypeQuery1"))
    (if _returnvalue_2
      (`|SpawnActorFromClass` (`KismetArrayLibrary.Array_Random` (`|MakeArray` "/Game/ThisProject/Enemy/BP_Cultist_1.BP_Cultist_1_C" "/Game/ThisProject/Enemy/BP_Cultist_2.BP_Cultist_2_C" :!type "Actor Class Reference")) (`KismetMathLibrary.MakeTransform` (`.ImpactPoint` (`GameplayStatics.BreakHitResult` _outhit))) "Undefined" "MultiplyWithRoot" null null))))

(event `self.Comp_Health.On Resource Emptied`
  ; Death
  (`self.Turn on Physics` false)
  (`self.Set Spin` 2.0)
  (`NiagaraFunctionLibrary.SpawnSystemAtLocation` "/Game/ThisProject/Assets_Imports/Character/Enemy/NS_HeadExplosion.NS_HeadExplosion" (`SceneComponent.K2_GetComponentLocation` (`self.Sphere1`)))
  (`ActorComponent.K2_DestroyComponent` (`self.WeakPoint`))
  (`self.Widget and Music` false)
  (`KismetSystemLibrary.MoveComponentTo` (`self.Box`) (+ (`self.Start Location`) (0.0 0.0 1000.0)) (struct) true true 10.0)
  (`NiagaraFunctionLibrary.SpawnSystemAtLocation` "/Game/ThisProject/Boss/NS_BossExplosion.NS_BossExplosion" (`SceneComponent.K2_GetComponentLocation` (`self.Box`)))
  (`self.K2_DestroyActor`)
  (message `/Game/ThisProject/Interactables/Power/BPI_Activate.Activate` (`self.Door`)))

(event `Set Spin`
  (params (Strength :type "Float (single-precision)"))
  (bind _returnvalue (* Strength 5.0))
  ; Spin
  (set `self.IsSpinning?` (!= Strength 0.0))
  (`Timeline|TL_Spin`
    (:`Update`
      (`SceneComponent.K2_AddWorldRotation` (`self.BossShell`) (`KismetMathLibrary.MakeRotator` 0.0 _returnvalue _returnvalue) false false))))

(event `Start Fight`
  ; Start Fight
  (`self.Widget and Music` true)
  (`KismetSystemLibrary.K2_SetTimerDelegate` (`|CreateDelegate` :!event `Attack`) 30.0 true)
  (`self.Attack`)
  (`KismetSystemLibrary.K2_SetTimerDelegate` (`|CreateDelegate` :!event `Spawn`) 60.0 true)
  (`self.Spawn`)
  (`KismetSystemLibrary.K2_SetTimerDelegate` (`|CreateDelegate` :!event `Check Player Distance`) 1.0 true))

(event `Change Locations`
  (bind _box (`self.Box`))
  ; Change Locations
  (`NiagaraFunctionLibrary.SpawnSystemAtLocation` "/Game/ThisProject/Boss/NS_BossTeleport.NS_BossTeleport" (+ (`SceneComponent.K2_GetComponentLocation` _box) (0.0 0.0 50.0)))
  (`SceneComponent.K2_SetWorldRotation` :`self` (`self.Box`))
  (if (`self.Is Stunned`)
    (`SceneComponent.K2_SetRelativeLocation` (`self.Box`) (`self.Start Location`) false false)
    (else
      (`SceneComponent.K2_SetRelativeLocation` _box (`self.Get Next Teleport`) false false))))

(event `Start Machine Gun Attack`
  ; Machine Gun Attack
  (`GameplayStatics.PlaySoundAtLocation` "/Game/ThisProject/SFX/MSS_GoldenButton.MSS_GoldenButton" (`SceneComponent.K2_GetComponentLocation` (`self.Box`)) (struct) 2.0 8.0 0.0 "/Game/ThisProject/SFX/SA_Large.SA_Large" null null null)
  (`self.Set Spin` 0.0)
  (`self.MachineGun`))

(event `self.Comp_Health.On Resource Lost`
  (params (Lost :type "Float (double-precision)"))
  (bind _comp_health (`self.Comp_Health`))
  ; On Damage Taken
  (`/Game/ThisProject/Boss/WB_BossHealthBar.Update` (`self.Health Bar`) (/ (`/Game/ThisProject/Comp_Resource.Current Resource` _comp_health) (`/Game/ThisProject/Comp_Resource.Max Resource` _comp_health)))
  (if (> Lost 9.0)
    (`self.Turn on Physics` true)
    (`KismetSystemLibrary.K2_SetTimerDelegate` (delegate `Get Back Up`) 15.0)))

(event `Attack`
  ; Machine Gun Attack
  (`self.Start Machine Gun Attack`))

(event `Get Back Up`
  ; On Damage Taken
  (set `self.Teleport Int` 0)
  (`self.Turn on Physics` false)
  (`self.Change Locations`))

(event `End Machine Gun Attack`
  ; Machine Gun Attack
  (`self.Set Spin` 1.0)
  (set `self.Machine Gun Timer` 1.0)
  (set `self.Machine Gun Amount` 0))

(event `MachineGun`
  ; Machine Gun Attack
  (`self.Check Not Spin and Not Stunned`)
  (if (== (`self.Machine Gun Amount`) 100)
    (`self.End Machine Gun Attack`)
    (else
      (`self.Machine Gun Attack`))))

(event `self.ReceiveBeginPlay`
  (bind _box (`self.Box`))
  ; Begin Play
  (set `self.Reset Location` (`SceneComponent.K2_GetComponentLocation` _box))
  (`SceneComponent.SetVisibility` _box false true)
  (`SceneComponent.K2_SetRelativeLocation` (`self.Box`) (`self.Start Location`) false false)
  (set `self.Target` (`GameplayStatics.GetPlayerCharacter` 0)))

(event `/Game/ThisProject/Interactables/Power/BPI_Activate.Activate`
  (`SceneComponent.SetVisibility` (`self.Box`) true true)
  (`self.Set Spin` 0.0)
  (`KismetSystemLibrary.MoveComponentTo` (`self.Box`) (0.0 0.0 0.0) (struct) true true 5.0)
  (`self.Start Fight`))

(fn `Apply Damage`
  (params (`Damage Info` :type "/Game/ThisProject/Struct_DamageHitResult Structure"))
  (returns (Success :type Boolean))
  (bind (_damage _hitresult _hittags) (break `/Game/ThisProject/Struct_DamageHitResult` `Damage Info`))
  (`/Game/ThisProject/Comp_Health.Apply Damage to Health` (`self.Comp_Health`) (make `/Game/ThisProject/Struct_DamageHitResult` (`KismetMathLibrary.SelectFloat` _damage (/ _damage 4.0) (`BlueprintGameplayTagLibrary.HasTag` _hittags (struct :`TagName` "DamageTypes.Explosive") true)) _hitresult _hittags))
  (return true))

(fn `Check Activation`
  (returns (`Is Active` :type Boolean))
  (return false))

(fn `Check Player Distance`
  (bind _returnvalue (`SceneComponent.K2_GetComponentLocation` (`self.Box`)))
  (bind _returnvalue_2 (`self.K2_GetActorLocation` (`self.Target`)))
  (if (< (`KismetMathLibrary.Vector_Distance` _returnvalue_2 _returnvalue) 300.0)
    (if (not (`self.Is Stunned`)) :!label _label
      (`self.Change Locations`))
    (elif (> (`KismetMathLibrary.Abs` (- (.z _returnvalue_2) (.z _returnvalue))) 500.0)
      (goto _label))))

(fn `Get Next Teleport`
  (returns (Output :type "Vector Structure"))
  (bind _teleport_int (`self.Teleport Int`))
  (if (== _teleport_int 3)
    (set `self.Teleport Int` 0)
    (return (`self.Start Location`))
    (else
      (`/Engine/EditorBlueprintResources/StandardMacros.IncrementInt` _teleport_int
        (:`  `
          (return (`|GetArrayItem` (`self.Teleport Locations`) _teleport_int)))))))

(fn `Get Target Look At Rotation`
  (returns (ReturnValue :type "Rotator Structure"))
  (return (`KismetMathLibrary.MakeRotator` 0.0 0.0 (+ (.yaw (`KismetMathLibrary.Conv_VectorToRotator` (`KismetMathLibrary.GetDirectionUnitVector` (`self.K2_GetActorLocation`) (`SceneComponent.K2_GetComponentLocation` (`Character.Mesh` (`self.Target`)))))) 90.0))))

(fn `Machine Gun Attack`
  (locals (`Gun Location` :type "Vector Structure" :default (0.0 0.0 0.0)))
  (bind _gun_location (`local.Gun Location`))
  (bind _returnvalue (`KismetMathLibrary.GetDirectionUnitVector` (`local.Gun Location`) (`SceneComponent.K2_GetComponentLocation` (`Character.Mesh` (`self.Target`)))))
  (set `local.Gun Location` (`SceneComponent.K2_GetComponentLocation` (`self.Gun`)))
  (bind (_outhit _returnvalue_2) (`KismetSystemLibrary.LineTraceSingle` _gun_location (`/Game/Base/BFL_General.Convert Trace` _gun_location _returnvalue 5000.0) "TraceTypeQuery1"))
  (if _returnvalue_2
    (bind (_outhit_2 _returnvalue_3) (`KismetSystemLibrary.LineTraceSingle` :`Start` (`local.Gun Location`) :`End` (`/Game/Base/BFL_General.Convert Trace` (`local.Gun Location`) _returnvalue 5000.0 10.0) :`TraceChannel` "TraceTypeQuery1" :`DrawDebugType` (`self.DebugMode`)))
    (bind (_bblockinghit _binitialoverlap _time _distance _location _impactpoint _normal _impactnormal _physmat _hitactor _hitcomponent _hitbonename _bonename _hititem _elementindex _faceindex _tracestart _traceend) (`GameplayStatics.BreakHitResult` _outhit_2))
    (`NiagaraFunctionLibrary.SpawnSystemAtLocation` "/Game/ThisProject/Boss/NS_BossProjectile.NS_BossProjectile" _tracestart (`KismetMathLibrary.Conv_VectorToRotator` (`KismetMathLibrary.GetDirectionUnitVector` _tracestart _traceend))))
  (set `self.Machine Gun Timer` (* (`self.Machine Gun Timer`) 0.8))
  (`KismetSystemLibrary.K2_SetTimerDelegate` (`|CreateDelegate` :!event `MachineGun`) (`KismetMathLibrary.FClamp` (`self.Machine Gun Timer`) 0.1))
  (`/Engine/EditorBlueprintResources/StandardMacros.IncrementInt` (`self.Machine Gun Amount`)
    (:`  `
      (if _returnvalue_3
        (`self.Machine Gun Damage` _outhit_2)))))

(fn `Machine Gun Damage`
  (params (InputPin :type "HitResult Structure"))
  (message `/Game/ThisProject/BPI_Health.Apply Damage` (`.HitActor` (`GameplayStatics.BreakHitResult` InputPin)) (make `/Game/ThisProject/Struct_DamageHitResult` 0.1 InputPin (struct :`GameplayTags` (struct :`(TagName` "DamageSource.Enemy")))))
  (`/Game/Base/BFL_General.Play Effect` InputPin))

(fn `Stop Widget anad Music`
  (`AudioComponent.Stop` (`self.Boss Music`))
  (`/Game/ThisProject/Boss/WB_BossHealthBar.Remove` (`self.Health Bar`)))

(fn `Turn on Physics`
  (params (bSimulate :type Boolean))
  (`PrimitiveComponent.SetSimulatePhysics` (`self.Box`) bSimulate)
  (`self.Set Spin` (`KismetMathLibrary.SelectFloat` 0.0 1.0 bSimulate))
  (set `self.Is Stunned` bSimulate))

(fn `UserConstructionScript`)

(fn `Widget and Music`
  (params (Activate :type Boolean))
  (if Activate
    (bind _returnvalue (`GameplayStatics.CreateSound2D` "/Game/ThisProject/Boss/MSS_BossMusic.MSS_BossMusic" 2.0 1.0 0.0 null))
    (bind _output_get (set `self.Boss Music` _returnvalue))
    (`AudioComponent.Play` _output_get 0.0)
    (bind _returnvalue_2 (`|CreateWidget` "/Game/ThisProject/Boss/WB_BossHealthBar.WB_BossHealthBar_C"))
    (bind _output_get_2 (set `self.Health Bar` _returnvalue_2))
    (`UserWidget.AddToViewport` _output_get_2 0)
    (else
      (`AudioComponent.Stop` (`self.Boss Music`))
      (`/Game/ThisProject/Boss/WB_BossHealthBar.Remove` (`self.Health Bar`)))))