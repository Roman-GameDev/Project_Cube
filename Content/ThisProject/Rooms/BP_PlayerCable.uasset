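; BP_PlayerCable is an interactable cable whose end can be picked up and dropped.
; Interacting attaches the cable to the interactor's component and resets the physics end onto Parent, or drops it if already held.
; A looping timer also triggers the drop when Parent exceeds cable length, using a DoOnce to detach, clamp position and enable physics.
; The plug sphere trace is a stub that always returns false.
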(event `Reset`
  (bind _returnvalue (`self.K2_GetActorLocation`))
  (bind _end (`self.End`))
  (bind _end_2 (`self.End`))
  (bind _returnvalue_2 (`SceneComponent.K2_GetComponentLocation` (`self.Parent`)))
  (`PrimitiveComponent.SetSimulatePhysics` (`self.End`) false)
  (`SceneComponent.K2_AttachToComponent` (`self.End`) (`self.Parent`) "None" "SnapToTarget" "SnapToTarget" "SnapToTarget" true)
  (goto _label :!via `Reset`))

(event `self.ReceiveBeginPlay`
  (`SceneComponent.K2_AttachToComponent` (`self.End`) (`self.Parent`) "None" "SnapToTarget" "SnapToTarget" "SnapToTarget" true)
  (`CableComponent.SetAttachEndToComponent` (`self.Cable`) (`self.End`) "None")
  (`KismetSystemLibrary.K2_SetTimerDelegate` (delegate `Check Distance`) 0.4 true))

(event `Drop`
  (bind _returnvalue (`self.K2_GetActorLocation`))
  (bind _end (`self.End`))
  (bind _end_2 (`self.End`))
  (bind _returnvalue_2 (`SceneComponent.K2_GetComponentLocation` (`self.Parent`)))
  (`/Engine/EditorBlueprintResources/StandardMacros.DoOnce` false :!label _label
    (:`Completed`
      (`SceneComponent.K2_DetachFromComponent` _end_2 "KeepWorld" "KeepWorld" "KeepWorld" true)
      (`CableComponent.SetAttachEndToComponent` (`self.Cable`) _end "None")
      (`SceneComponent.K2_SetWorldTransform` (`self.End`) (`KismetMathLibrary.MakeTransform` (`KismetMathLibrary.SelectVector` (+ _returnvalue (* (`KismetMathLibrary.GetDirectionUnitVector` _returnvalue _returnvalue_2) (- (`self.Cable Length`) 45.0))) _returnvalue_2 (> (`KismetMathLibrary.Vector_Distance` (`SceneComponent.K2_GetComponentLocation` (`self.Parent`)) (`SceneComponent.K2_GetComponentLocation` (`self.Cable`))) (`self.Cable Length`)))) false false)
      (`PrimitiveComponent.SetSimulatePhysics` _end_2 true)
      (`PrimitiveComponent.SetPhysicsLinearVelocity` _end (0.0 0.0 0.0) false "None"))))

(event `Check Distance`
  (if (> (`KismetMathLibrary.Vector_Distance` (`SceneComponent.K2_GetComponentLocation` (`self.Parent`)) (`SceneComponent.K2_GetComponentLocation` (`self.Cable`))) (`self.Cable Length`))
    (goto _label)))

(fn `Interact`
  (params (Interactor :type "Actor Object Reference") (`Interacting Component` :type "SceneComponent Object Reference"))
  (returns (Success :type Boolean))
  (if (`self.IsHeld`)
    (bind _success (`self.Trace For Plugs`))
    (if (not _success)
      (`self.Drop`)
      (set `self.IsHeld` false))
    (else
      (set `self.IsHeld` true)
      (`self.Reset`)
      (`CableComponent.SetAttachEndToComponent` (`self.Cable`) `Interacting Component` "None")
      (return false))))

(fn `Trace For Plugs`
  (returns (Success :type Boolean))
  (bind _returnvalue (`SceneComponent.K2_GetComponentLocation` (`self.End`)))
  (`KismetSystemLibrary.SphereTraceSingle` :`Start` _returnvalue :`End` (- _returnvalue (0.0 0.0 1.0)) :`Radius` 35.0 :`TraceChannel` "TraceTypeQuery6" :`DrawDebugType` "ForDuration")
  (return false))

(fn `UserConstructionScript`
  (locals (`Last Cable End` :type "Transform Structure")))