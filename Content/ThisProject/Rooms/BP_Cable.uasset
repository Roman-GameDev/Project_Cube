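; BP_Cable is a room actor that builds a chain of hanging cables through a list of end-point transforms.
; Each segment starts at the previous point, or the actor origin, and attaches to a spawned static mesh placed at the next point, clamped to the maximum cable length.
; The View flag generates cables in the construction script instead of at BeginPlay.
; The construction script also attaches the actor to an optional parent, keeping world transform.
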(event `self.ReceiveBeginPlay`
  (if (not (`self.View`))
    (`self.Generate Cables`)))

(event `Generate Cables`
  (bind _cable_ends (`self.Cable Ends`))
  (bind _cable_max_length (`self.Cable Max Length`))
  (`AddComponent|NODE_AddStaticMeshComponent-4`)
  (for _index (range (`KismetArrayLibrary.Array_Length` (`self.Cable Ends`)))
    (bind _returnvalue (- _index 1))
    (bind _returnvalue_2 (`AddComponent|NODE_AddCableComponent-1` :`RelativeTransform` (`KismetMathLibrary.SelectTransform` (`KismetMathLibrary.MakeTransform` (0.0 0.0 0.0)) (`|GetArrayItem` (`self.Cable Ends`) _returnvalue) (== _returnvalue -1))))
    (bind _location (.location (`|GetArrayItem` _cable_ends _index)))
    (bind _returnvalue_3 (- _index 1))
    (bind _location_2 (.location (`KismetMathLibrary.SelectTransform` (`KismetMathLibrary.MakeTransform` (0.0 0.0 0.0)) (`|GetArrayItem` _cable_ends _returnvalue_3) (== _returnvalue_3 -1))))
    (bind _returnvalue_4 (`AddComponent|NODE_AddStaticMeshComponent-2` :`RelativeTransform` (`KismetMathLibrary.MakeTransform` (`KismetMathLibrary.SelectVector` _location (+ (* (`KismetMathLibrary.GetDirectionUnitVector` _location_2 _location) _cable_max_length) _location_2) (<= (`KismetMathLibrary.Vector_Distance` _location _location_2) _cable_max_length)) (.rotation (`KismetMathLibrary.SelectTransform` (`KismetMathLibrary.MakeTransform` (0.0 0.0 0.0)) (`|GetArrayItem` _cable_ends _returnvalue_3) (== _returnvalue_3 -1))) (.scale (`KismetMathLibrary.SelectTransform` (`KismetMathLibrary.MakeTransform` (0.0 0.0 0.0)) (`|GetArrayItem` _cable_ends _returnvalue_3) (== _returnvalue_3 -1))))))
    (`CableComponent.SetAttachEndToComponent` _returnvalue_2 _returnvalue_4 "None")
    (set `CableComponent.CableLength` (`self.Cable Max Length`) _returnvalue_2)))

(fn `UserConstructionScript`
  (locals (`Last Cable End` :type "Transform Structure"))
  (`|ExecutionSequence`
    (:`then_0`
      (bind _parent_actor (`self.Parent Actor`)
        (:`then`
          (`self.K2_AttachToActor` _parent_actor "None" "KeepWorld" "KeepWorld" "KeepWorld"))
        (:`else`)))
    (:`then_1`
      (if (`self.View`)
        (`self.Generate Cables`)))))