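; BP_Note is a note actor that displays its text in the world and opens it on screen when interacted with.
; Construction Script and BeginPlay both push the Text variable into the WB_Note shown by its Widget component.
; Interact creates a WB_NoteWidget with the same text and exit keys, adds it to the viewport and returns true.
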(event `self.ReceiveBeginPlay`
  (bind _aswb_note (cast `/Game/ThisProject/Rooms/Note/WB_Note` (`WidgetComponent.GetWidget` (`self.Widget`))))
  (`/Game/ThisProject/Rooms/Note/WB_Note.Update Text` _aswb_note (`self.Text`)))

(fn `Interact`
  (params (Interactor :type "Actor Object Reference") (`Interacting Component` :type "SceneComponent Object Reference"))
  (returns (Success :type Boolean))
  (bind _returnvalue (`|CreateWidget` "/Game/ThisProject/Rooms/Note/WB_NoteWidget.WB_NoteWidget_C" null (`self.Text`) (`|MakeArray` "Escape" "E" :!type "Key Structure")))
  (`UserWidget.AddToViewport` _returnvalue 0)
  (return true))

(fn `UserConstructionScript`
  (bind _aswb_note (cast `/Game/ThisProject/Rooms/Note/WB_Note` (`WidgetComponent.GetWidget` (`self.Widget`))))
  (`/Game/ThisProject/Rooms/Note/WB_Note.Update Text` _aswb_note (`self.Text`)))