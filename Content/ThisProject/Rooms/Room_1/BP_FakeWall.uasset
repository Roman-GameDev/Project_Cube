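; BP_FakeWall is a Room 1 wall actor that topples over once when activated.
; BeginPlay stores the starting rotation and scales the Fall timeline's play rate so the fall lasts the configured Seconds.
; Activate passes through a DoOnce and plays the timeline, whose alpha lerps the actor's rotation from the start to the Fallen rotation.
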(event `self.ReceiveBeginPlay`
  (set `self.Start` (`self.K2_GetActorRotation`))
  (`TimelineComponent.SetPlayRate` (`self.Fall`) (/ 1.0 (`self.Seconds`))))

(event `/Game/ThisProject/Interactables/Power/BPI_Activate.Activate`
  (`/Engine/EditorBlueprintResources/StandardMacros.DoOnce` false
    (:`Completed`
      (bind (_direction _alpha) (`Timeline|Fall` :!via `PlayFromStart`)
        (:`Update`
          (`self.K2_SetActorRotation` (`KismetMathLibrary.RLerp` (`self.Start`) (`self.Fallen`) _alpha)))))))

(fn `UserConstructionScript`)