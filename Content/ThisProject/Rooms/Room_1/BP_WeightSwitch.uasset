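; BP_WeightSwitch is a pressure switch in Room 1 that stays active while anything overlaps its Box.
; The first overlap sets IsToggled, forces DynamicStaticMesh to its end position and calls Trigger on every entry in Triggerables.
; When the Box has no overlapping components left, it clears the flag, returns the mesh to its start and calls Untrigger on each entry.
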(event `self.Box.OnComponentBeginOverlap`
  (params (OverlappedComponent :type "PrimitiveComponent Object Reference") (OtherActor :type "Actor Object Reference") (OtherComp :type "PrimitiveComponent Object Reference") (OtherBodyIndex :type Integer) (bFromSweep :type Boolean) (SweepResult :type "HitResult Structure (by ref)"))
  (if (not (`self.IsToggled?`))
    (set `self.IsToggled?` true)
    (`/Game/ThisProject/Rooms/Dynamic_Static_Mesh.Force Move to End` (`self.Dynamic_Static_Mesh`))
    (for _array_element (`self.Triggerables`)
      (`/Game/ThisProject/Rooms/Room_1/BP_ButtonTriggerables.Trigger` _array_element))))

(event `self.Box.OnComponentEndOverlap`
  (params (OverlappedComponent :type "PrimitiveComponent Object Reference") (OtherActor :type "Actor Object Reference") (OtherComp :type "PrimitiveComponent Object Reference") (OtherBodyIndex :type Integer))
  (if (`KismetArrayLibrary.Array_IsEmpty` (`PrimitiveComponent.GetOverlappingComponents` (`self.Box`)))
    (set `self.IsToggled?` false)
    (`/Game/ThisProject/Rooms/Dynamic_Static_Mesh.Force Move to Start` (`self.Dynamic_Static_Mesh`))
    (for _array_element (`self.Triggerables`)
      (`/Game/ThisProject/Rooms/Room_1/BP_ButtonTriggerables.Untrigger` _array_element))))

(fn `UserConstructionScript`)