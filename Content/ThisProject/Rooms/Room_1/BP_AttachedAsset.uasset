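; BP_AttachedAsset is a configurable Room 1 prop that shows a mesh, plays a sound and can take damage.
; Its construction script applies the chosen mesh and attaches the actor to a parent actor, keeping world transform.
; On BeginPlay it spawns the sound attached to the mesh.
; ApplyDamage forwards damage info to its health component and always returns false.
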(event `self.ReceiveBeginPlay`
  (`GameplayStatics.SpawnSoundAttached` (`self.Sound`) (`self.StaticMesh`) "None" (0.0 0.0 0.0) (struct) "KeepRelativeOffset" false 1.0 1.0 0.0 null null))

(fn `Apply Damage`
  (params (`Damage Info` :type "/Game/ThisProject/Struct_DamageHitResult Structure"))
  (returns (Success :type Boolean))
  (`/Game/ThisProject/Comp_Health.Apply Damage to Health` (`self.Comp_Health`) `Damage Info`)
  (return false))

(fn `UserConstructionScript`
  (`StaticMeshComponent.SetStaticMesh` (`self.StaticMesh`) (`self.Mesh`))
  (`self.K2_AttachToActor` (`self.Parent Actor`) "None" "KeepWorld" "KeepWorld" "KeepWorld"))