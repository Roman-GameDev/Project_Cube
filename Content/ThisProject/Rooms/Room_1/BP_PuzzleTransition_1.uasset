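; Room 1 puzzle transition trigger that introduces the first cultist enemy once it has been activated.
; When the player enters the box, it spawns the cultist once at the Cultist component's transform and starts its intro voiceline.
; It binds to the cultist's aggro event and, after a delay, has the GameInstance play Doug's enemy line.
; A separate one-shot NextVoiceline event plays the cultist's second intro line.
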(event `/Game/ThisProject/Interactables/Power/BPI_Activate.Activate`
  (set `self.Activated?` true))

(event `self.Box.OnComponentBeginOverlap`
  (params (OverlappedComponent :type "PrimitiveComponent Object Reference") (OtherActor :type "Actor Object Reference") (OtherComp :type "PrimitiveComponent Object Reference") (OtherBodyIndex :type Integer) (bFromSweep :type Boolean) (SweepResult :type "HitResult Structure (by ref)"))
  (if (and (== OtherActor (`GameplayStatics.GetPlayerCharacter` 0)) (`self.Activated?`))
    (`/Engine/EditorBlueprintResources/StandardMacros.DoOnce` false
      (:`Completed`
        (bind _returnvalue (`|SpawnActorFromClass` "/Game/ThisProject/Enemy/BP_Cultist_First.BP_Cultist_First_C" (`SceneComponent.K2_GetComponentToWorld` (`self.Cultist`)) "AlwaysSpawn" "MultiplyWithRoot" null null))
        (set `self.Cultist Ref` _returnvalue)
        (`/Game/ThisProject/Enemy/BP_Enemy.Play Voiceline` _returnvalue "/Game/ThisProject/Enemy/Cubehead_Intro1.Cubehead_Intro1" true)
        (add `/Game/ThisProject/Enemy/BP_Enemy.On Aggroed` _returnvalue (`|CreateDelegate` :!event `Next Voiceline`))
        (`KismetSystemLibrary.Delay` 6.0)
        (message `/Game/ThisProject/Player/BPI_GameInstance.Play Doug Line` (`GameplayStatics.GetGameInstance`) "/Game/ThisProject/Assets_Imports/Doug/Voicelines/Done/Doug_Enemy.Doug_Enemy")))))

(event `Next Voiceline`
  (`/Engine/EditorBlueprintResources/StandardMacros.DoOnce` false
    (:`Completed`
      (`/Game/ThisProject/Enemy/BP_Enemy.Play Voiceline` (`self.Cultist Ref`) "/Game/ThisProject/Enemy/Cubehead_intro2.Cubehead_intro2" true))))

(fn `Check Activation`
  (returns (`Is Active` :type Boolean))
  (return false))

(fn `UserConstructionScript`)