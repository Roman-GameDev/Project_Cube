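; BP_Timer is a countdown clock actor in Room 1 that shows remaining time on a WB_Clock widget component.
; BeginPlay caches the clock widget and starts a looping one-second timer.
; The Tick event alternates tick and tock sounds at the actor's location via a FlipFlop, decrements Seconds and passes minutes and seconds to the widget.
; Activate destroys the actor, and the graph has no zero-time check.
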(event `self.ReceiveBeginPlay`
  (bind _aswb_clock (cast `/Game/ThisProject/Rooms/Room_1/WB_Clock` (`WidgetComponent.GetWidget` (`self.Widget`))))
  (set `self.Clock` _aswb_clock)
  (`KismetSystemLibrary.K2_SetTimerDelegate` (`|CreateDelegate` :!event `Tick`) 1.0 true))

(event `Tick`
  (`/Engine/EditorBlueprintResources/StandardMacros.FlipFlop`
    (:`A`
      (`GameplayStatics.PlaySoundAtLocation` "/Game/ThisProject/SFX/MSS_Tick.MSS_Tick" (`self.K2_GetActorLocation`) (struct) 1.0 1.0 0.0 null null null null))
    (:`B`
      (`GameplayStatics.PlaySoundAtLocation` "/Game/ThisProject/SFX/MSS_Tock.MSS_Tock" (`self.K2_GetActorLocation`) (struct) 1.0 1.0 0.0 null null null null)))
  (bind _result (`/Engine/EditorBlueprintResources/StandardMacros.DecrementInt` (`self.Seconds`))
    (:`  `
      (`/Game/ThisProject/Rooms/Room_1/WB_Clock.Update Time` (`self.Clock`) (/ _result 60) (mod _result 60)))))

(event `/Game/ThisProject/Interactables/Power/BPI_Activate.Activate`
  (`self.K2_DestroyActor`))

(fn `UserConstructionScript`)