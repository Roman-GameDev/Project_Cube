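; BP_TheButton_Room1 is the Room 1 version of a triggerable button, adding a walls-falling sound to its inherited behavior.
; Its Trigger event runs the parent logic, then passes through a DoOnce so the extra effect fires only on the first trigger.
; After a short delay, it plays the Room 1 walls-falling sound at the button's own location.
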(event `self.Trigger`
  (`parent.Trigger`)
  (`/Engine/EditorBlueprintResources/StandardMacros.DoOnce` false
    (:`Completed`
      (`KismetSystemLibrary.Delay` 0.5)
      (`GameplayStatics.PlaySoundAtLocation` "/Game/ThisProject/SFX/MSS_Room1_WallsFalling.MSS_Room1_WallsFalling" (`self.K2_GetActorLocation`) (struct) 1.0 1.0 0.0 null null null null))))

(fn `UserConstructionScript`
  (`parent.UserConstructionScript`))