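; BP_Door is a door actor that opens and closes by moving its DynamicStaticMesh between start and end positions.
; Trigger opens it, unless it requires power and is unpowered, while Untrigger always closes it.
; PowerSignal only updates the powered state, without moving the door.
; The construction script passes end position and time to the mesh, then applies the StartOpen state.
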(event `Open`
  (`/Game/ThisProject/Rooms/Dynamic_Static_Mesh.Force Move to End` (`self.Dynamic_Static_Mesh`)))

(event `Close`
  (`/Game/ThisProject/Rooms/Dynamic_Static_Mesh.Force Move to Start` (`self.Dynamic_Static_Mesh`)))

(event `self.Trigger`
  (if (`self.RequiresPower?`)
    (if (`self.IsPowered?`)
      (`self.Open` :!label _label))
    (else
      (goto _label))))

(event `self.Untrigger`
  (`self.Close`))

(event `/Game/ThisProject/Interactables/Power/BPI_Power.Power Signal`
  (params (`Powered?` :type Boolean))
  (set `self.IsPowered?` `Powered?`))

(fn `UserConstructionScript`
  (bind _dynamic_static_mesh (`self.Dynamic_Static_Mesh`))
  (`parent.UserConstructionScript`)
  (set `/Game/ThisProject/Rooms/Dynamic_Static_Mesh.End Position` (`self.End Position`) _dynamic_static_mesh)
  (set `/Game/ThisProject/Rooms/Dynamic_Static_Mesh.Time` (`self.Time`) _dynamic_static_mesh)
  (if (`self.Start Open?`)
    (`self.Open`)
    (else
      (`self.Close`))))